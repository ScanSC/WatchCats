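; Computer Blueprint for level 2's win condition, offering a command interface and returning the game to the main menu when finished.
; ManageCommand dispatches command names to Help, Clear, List Devices, Activate, Notes Mem and Destroy Virus handlers, passing the parameter only to Activate.
; Tick calls the parent and polls IsFinished, which is set outside these graphs, then opens L_MainMenu after a 15-second delay.
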(event `self.ReceiveTick`
  (params (DeltaSeconds :type "Float (single-precision)"))
  (`parent.ReceiveTick` DeltaSeconds)
  (if (`self.IsFinished`)
    (`KismetSystemLibrary.Delay` 15.0)
    (`GameplayStatics.OpenLevel` "L_MainMenu")))

(fn `Manage Command`
  (params (CommandName :type String) (Parameter :type String))
  (switch `string` CommandName
    (:`Help`
      (`self.CommandHelp`))
    (:`Clear`
      (`self.CommandClear`))
    (:`ListDevices`
      (`self.CommandListDevices`))
    (:`Activate`
      (`self.CommandActivate` Parameter))
    (:`NotesMem`
      (`self.CommandNotesMem`))
    (:`DestroyVirus`
      (`self.CommandDestroyVirus`))))

(fn `UserConstructionScript`
  (`parent.UserConstructionScript`))