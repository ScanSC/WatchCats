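; Possessable computer camera that the player can hack, with a text terminal for controlling connected devices.
; BeginPlay creates the terminal and camera-swap widgets, which possession and swap functions show or hide.
; ManageCommand routes typed input to help, clear, device listing, activation by name and notes commands, printing replies to the terminal.
; Cursor hover outlines the mesh by hacked state, and construction generates a random numeric name.
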(event `self.ReceiveBeginPlay`
  (`parent.ReceiveBeginPlay`)
  (`|ExecutionSequence`
    (:`then_0`
      (bind _returnvalue (`|CreateWidget` "/Game/Cameras/CamerasLib/Computer/WBP_Terminal.WBP_Terminal_C"))
      (bind _output_get (set `self.Terminal` _returnvalue))
      (set `/Game/Cameras/CamerasLib/Computer/WBP_Terminal.Computer` self _output_get))
    (:`then_1`
      (bind _returnvalue_2 (`|CreateWidget` "/Game/Cameras/CamerasLib/Computer/WBP_ComputerSwap.WBP_ComputerSwap_C"))
      (set `self.CameraSwapHUD` _returnvalue_2))))

(event `self.DetectionBox.OnBeginCursorOver`
  (params (TouchedComponent :type "PrimitiveComponent Object Reference"))
  ;[1 1 1] set object highlight
  (`self.Highlight Object` (`|MakeArray` (`self.Computer`) :!type "MeshComponent Object Reference") (select `bool` (`self.HasBeenHacked?`) :`false` "/Game/Cameras/Materials/M_Outline_NotHackedCamera_Inst.M_Outline_NotHackedCamera_Inst" :`true` "/Game/Cameras/Materials/M_Outline_HackedCamera_Inst.M_Outline_HackedCamera_Inst" :!type "MaterialInstance Object Reference")))

(event `self.DetectionBox.OnEndCursorOver`
  (params (TouchedComponent :type "PrimitiveComponent Object Reference"))
  ;[1 1 1] unset highlight
  (`self.Highlight Object` (`|MakeArray` (`self.Computer`) :!type "MeshComponent Object Reference")))

(fn `CommandActivate`
  (params (Parameter :type String))
  (if (`KismetStringLibrary.IsEmpty` Parameter)
    (`/Game/Cameras/CamerasLib/Computer/WBP_Terminal.Add_line` (`self.Terminal`) "Usage: Activate <Device_Name>" false)
    (else
      (for _array_element (`self.ConnectedDevices`)
        (if (`KismetStringLibrary.EqualEqual_StrStr` Parameter (`/Game/Level/Props/BP_AbstractConnectedDevice.Name` _array_element))
          (`/Game/Level/Props/BP_AbstractConnectedDevice.Activate` _array_element)
          (`/Game/Cameras/CamerasLib/Computer/WBP_Terminal.Add_line` (`self.Terminal`) (`KismetStringLibrary.Concat_StrStr` (`KismetStringLibrary.Concat_StrStr` "Device \"" Parameter) "\" activated.") false)
          (`KismetSystemLibrary.PrintString` "cinematic")
          (return))))))

(fn `CommandClear`
  (bind _terminal (`self.Terminal`))
  (`KismetArrayLibrary.Array_Clear` (`/Game/Cameras/CamerasLib/Computer/WBP_Terminal.Lines` _terminal))
  (`/Game/Cameras/CamerasLib/Computer/WBP_Terminal.Add_line` _terminal "Command lines cleared" false))

(fn `CommandError`
  (params (CommandName :type String))
  (`/Game/Cameras/CamerasLib/Computer/WBP_Terminal.Add_line` (`self.Terminal`) (`KismetStringLibrary.Concat_StrStr` (`KismetStringLibrary.Concat_StrStr` (`KismetStringLibrary.Concat_StrStr` "\"" CommandName) "\"") ": Unrecognized Command. For command list type \"help\".") false))

(fn `CommandHelp`
  (for _array_element (`self.CommandList`)
    (`/Game/Cameras/CamerasLib/Computer/WBP_Terminal.Add_line` (`self.Terminal`) (`KismetStringLibrary.Concat_StrStr` (`KismetStringLibrary.Concat_StrStr` (break `/Game/Cameras/CamerasLib/Computer/Struct_Commands` _array_element) " : ") (`.Description_8_0473AD014E06234DE09E0E85772B52FC` (break `/Game/Cameras/CamerasLib/Computer/Struct_Commands` _array_element))) false)))

(fn `CommandListDevices`
  (if (`KismetArrayLibrary.Array_IsEmpty` (`self.ConnectedDevices`))
    (`/Game/Cameras/CamerasLib/Computer/WBP_Terminal.Add_line` (`self.Terminal`) "No connected devices." false)
    (else
      (`/Game/Cameras/CamerasLib/Computer/WBP_Terminal.Add_line` (`self.Terminal`) "Connected devices :" false)
      (for _array_element (`self.ConnectedDevices`)
        (`/Game/Cameras/CamerasLib/Computer/WBP_Terminal.Add_line` (`self.Terminal`) (`/Game/Level/Props/BP_AbstractConnectedDevice.Name` _array_element) false)))))

(fn `CommandNotesMem`
  (`/Game/Cameras/CamerasLib/Computer/WBP_Terminal.Add_line` (`self.Terminal`) "Notes memory :" false)
  (`/Game/Cameras/CamerasLib/Computer/WBP_Terminal.Add_line` (`self.Terminal`) (`self.NotesMemory`) false))

(fn `GenerateComputerName`
  (set `self.ComputerName` (`KismetStringLibrary.Concat_StrStr` (`KismetStringLibrary.Concat_StrStr` (`KismetStringLibrary.Conv_IntToString` (`KismetMathLibrary.RandomInteger` 9)) (`KismetStringLibrary.Conv_IntToString` (`KismetMathLibrary.RandomInteger` 9))) (`KismetStringLibrary.Concat_StrStr` "." (`KismetStringLibrary.Conv_IntToString` (`KismetMathLibrary.RandomInteger` 9))))))

(fn `ManageCommand`
  (params (Input :type String))
  (bind _returnvalue (`KismetStringLibrary.FindSubstring` Input " "))
  (bind _returnvalue_2 (== _returnvalue -1))
  (bind _returnvalue_3 (select `bool` _returnvalue_2 :`false` (`KismetStringLibrary.Left` Input _returnvalue) :`true` Input))
  ;[1 1 1] Do nothing if command empty
  (if (not (`KismetStringLibrary.IsEmpty` Input))
    (switch `string` _returnvalue_3
      (:`Default`
        (`self.CommandError` _returnvalue_3))
      (:`help`
        (`self.CommandHelp`))
      (:`Clear`
        (`self.CommandClear`))
      (:`ListDevices`
        (`self.CommandListDevices`))
      (:`Activate`
        (`self.CommandActivate` (`KismetStringLibrary.Trim` (select `bool` _returnvalue_2 :`false` (`KismetStringLibrary.RightChop` Input _returnvalue)))))
      (:`NotesMem`
        (`self.CommandNotesMem`)))))

(fn `PossessCamera`
  (`parent.PossessCamera`)
  (`UserWidget.AddToViewport` (`self.CameraSwapHUD`) 1))

(fn `SwapToCamera`
  (`Widget.RemoveFromParent` (`self.Terminal`)))

(fn `SwapToTerminal`
  (`UserWidget.AddToViewport` (`self.Terminal`) 0))

(fn `UnpossessCamera`
  (`parent.UnpossessCamera`)
  (`self.SwapToCamera`)
  (`Widget.RemoveFromParent` (`self.CameraSwapHUD`)))

(fn `UserConstructionScript`
  (`parent.UserConstructionScript`)
  (`self.GenerateComputerName`))