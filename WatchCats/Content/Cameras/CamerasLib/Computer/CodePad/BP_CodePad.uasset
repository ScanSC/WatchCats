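; BP_CodePad is an elevator terminal, a child of a camera-possessable computer, with an "Elevator-" name prefix and help, clear, infos and navigate commands.
; Infos prints status and the Floors map, while navigate validates the requested floor against it.
; NavigateTo activates the departure and destination doors, plays a sound, teleports the actor and updates the current floor.
; Its first possession starts the GameInstance's security alert.
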(fn `CommandInfos`
  (bind _floors (`self.Floors`))
  (`/Game/Cameras/CamerasLib/Computer/WBP_Terminal.Add_line` (`self.Terminal`) "------------" false)
  (`/Game/Cameras/CamerasLib/Computer/WBP_Terminal.Add_line` (`self.Terminal`) "Status : OK" false)
  (`/Game/Cameras/CamerasLib/Computer/WBP_Terminal.Add_line` (`self.Terminal`) "------------" false)
  (bind _keys (`BlueprintMapLibrary.Map_Keys` _floors))
  (for _array_element _keys
    (`/Game/Cameras/CamerasLib/Computer/WBP_Terminal.Add_line` (`self.Terminal`) (`KismetStringLibrary.Concat_StrStr` (`KismetStringLibrary.Concat_StrStr` (`KismetStringLibrary.Conv_IntToString` _array_element) " : ") (break `/Game/Cameras/CamerasLib/Computer/CodePad/Struct_FloorInformation` (`BlueprintMapLibrary.Map_Find` _floors _array_element))) false))
  (`/Game/Cameras/CamerasLib/Computer/WBP_Terminal.Add_line` (`self.Terminal`) "------------" false)
  (`/Game/Cameras/CamerasLib/Computer/WBP_Terminal.Add_line` (`self.Terminal`) (`KismetStringLibrary.Concat_StrStr` "Actual Floor : " (`KismetStringLibrary.Conv_IntToString` (`self.ActualFloor`))) false)
  (`/Game/Cameras/CamerasLib/Computer/WBP_Terminal.Add_line` (`self.Terminal`) "------------" false)
  (`/Game/Cameras/CamerasLib/Computer/WBP_Terminal.Add_line` (`self.Terminal`) "Last Update : 08/07/23" false)
  (`/Game/Cameras/CamerasLib/Computer/WBP_Terminal.Add_line` (`self.Terminal`) "Last Maintenance : 10/09/24" false))

(fn `CommandNavigate`
  (params (Parameter :type String))
  (bind _returnvalue (`KismetStringLibrary.Conv_StringToInt` Parameter))
  (if (`KismetStringLibrary.IsEmpty` Parameter)
    (`/Game/Cameras/CamerasLib/Computer/WBP_Terminal.Add_line` (`self.Terminal`) "Usage: navigate <floor>." false)
    (elif (`KismetStringLibrary.IsNumeric` Parameter)
      (if (`.ReturnValue` (`BlueprintMapLibrary.Map_Find` (`self.Floors`) _returnvalue))
        (if (!= _returnvalue (`self.ActualFloor`))
          (`self.NavigateTo` _returnvalue)
          (`/Game/Cameras/CamerasLib/Computer/WBP_Terminal.Add_line` (`self.Terminal`) (`KismetStringLibrary.Concat_StrStr` "Going to floor " Parameter) false)
          (else
            (`/Game/Cameras/CamerasLib/Computer/WBP_Terminal.Add_line` (`self.Terminal`) "Given floor is already the actual floor." false)))
        (else
          (`/Game/Cameras/CamerasLib/Computer/WBP_Terminal.Add_line` (`self.Terminal`) "Parameter must be a valid floor." false)))
      (else
        (`/Game/Cameras/CamerasLib/Computer/WBP_Terminal.Add_line` (`self.Terminal`) "Parameter must be an number." false)))))

(fn `GenerateComputerName`
  (`parent.GenerateComputerName`)
  (set `self.ComputerName` (`KismetStringLibrary.Concat_StrStr` "Elevator-" (`self.ComputerName`))))

(fn `Manage Command`
  (params (CommandName :type String) (Parameter :type String))
  (switch `string` CommandName
    (:`Default`
      (`self.CommandError` CommandName))
    (:`help`
      (`self.CommandHelp`))
    (:`Clear`
      (`self.CommandClear`))
    (:`Infos`
      (`self.CommandInfos`))
    (:`Navigate`
      (`self.CommandNavigate` Parameter))))

(fn `NavigateTo`
  (params (NewFloor :type Integer))
  (bind _floors (`self.Floors`))
  (bind _actualfloor (`self.ActualFloor`))
  (bind _value (`BlueprintMapLibrary.Map_Find` _floors NewFloor))
  (bind _keys (`BlueprintMapLibrary.Map_Keys` _floors))
  (for _array_element _keys
    (if (== NewFloor _array_element)
      (`/Game/Level/Props/BP_AbstractConnectedDevice.Activate` (`.Door_8_3B89B3924422FE816DE440BE342C055E` (break `/Game/Cameras/CamerasLib/Computer/CodePad/Struct_FloorInformation` _value)))
      (`GameplayStatics.PlaySound2D` "/Game/SFX/Elevator.Elevator" 1.0 1.0 0.0 null null)
      (`self.K2_TeleportTo` (`.Coordinate_5_3656233F410B879ECE59D6BDD55800DC` (break `/Game/Cameras/CamerasLib/Computer/CodePad/Struct_FloorInformation` _value)) (`SceneComponent.K2_GetComponentRotation` (`self.DefaultSceneRoot`)))
      (elif (== _array_element _actualfloor)
        (`/Game/Level/Props/BP_AbstractConnectedDevice.Activate` (`.Door_8_3B89B3924422FE816DE440BE342C055E` (break `/Game/Cameras/CamerasLib/Computer/CodePad/Struct_FloorInformation` (`BlueprintMapLibrary.Map_Find` _floors _actualfloor)))))))
  (set `self.ActualFloor` NewFloor))

(fn `PossessCamera`
  (`parent.PossessCamera`)
  (`/Engine/EditorBlueprintResources/StandardMacros.DoOnce` false
    (:`Completed`
      (bind _asbp_game_instance (cast `/Game/BP_GameInstance` (`GameplayStatics.GetGameInstance`)))
      (`/Game/BP_GameInstance.StartSecurityAlert` _asbp_game_instance))))

(fn `UserConstructionScript`
  (`parent.UserConstructionScript`))