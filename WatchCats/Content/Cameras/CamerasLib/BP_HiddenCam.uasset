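; BP_HiddenCam is a possessable camera named "Hidden Camera" that adds a joke line when the player takes control of it.
; It extends a parent camera class, setting its display name and using its Cube as the mesh to outline in the construction script.
; Its PossessCamera override runs the parent logic, then uses a DoOnce to show a timed spying quip through the game instance's DialogBox on first possession.
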(fn `PossessCamera`
  (`parent.PossessCamera`)
  (`/Engine/EditorBlueprintResources/StandardMacros.DoOnce` false
    (:`Completed`
      (bind _asbp_game_instance (cast `/Game/BP_GameInstance` (`GameplayStatics.GetGameInstance`)))
      (`/Game/Text/WBP_Dialog_Box.ShowDialogBox` (`/Game/BP_GameInstance.DialogBox` _asbp_game_instance) 4.0 "Hehe, Looks like someone is being spied on by their superiors."))))

(fn `UserConstructionScript`
  (`parent.UserConstructionScript`)
  (set `self.MeshToOutline` (`|MakeArray` (`self.Cube`) :!type "MeshComponent Object Reference"))
  (set `self.Name` "Hidden Camera"))