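; BP_SecurityCamOld is a security camera that the player rotates with look input.
; IA_Look input is converted into rotation modifiers and constrained, then yaw is applied to RotatorMesh and inverted pitch to CameraMesh.
; GetCameraRotation reads those two relative rotations back, and GetCamera returns Camera1.
; The construction script registers the arm and camera meshes in MeshToOutline.
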(event `EnhancedInput|/Game/Cameras/Inputs/InputActions/IA_Look`
  (params (ActionValue :type "Vector2D Structure") (ElapsedSeconds :type "Float (double-precision)") (TriggeredSeconds :type "Float (double-precision)") (InputAction :type "InputAction Object Reference" :default "/Game/Cameras/Inputs/InputActions/IA_Look.IA_Look"))
  ;[1 1 1] Look Input Event: rotate camera
  (:`Triggered`
    (bind (_xout _yout) (`self.GetRotationModifier` ActionValue_X ActionValue_Y))
    (bind (_newhorizontalrotation _newverticalrotation) (`self.ContraintViewModifiers` _xout _yout))
    (`SceneComponent.K2_SetRelativeRotation` (`self.RotatorMesh`) (`KismetMathLibrary.MakeRotator` 0.0 0.0 _newhorizontalrotation) true false)
    (`SceneComponent.K2_SetRelativeRotation` (`self.CameraMesh`) (`KismetMathLibrary.MakeRotator` 0.0 (* _newverticalrotation -1.0)) true false)))

(fn `GetCamera`
  (returns (Camera :type "CameraComponent Object Reference"))
  (return (`self.Camera1`)))

(fn `GetCameraRotation`
  (returns (HorizontalRotation :type "Float (double-precision)") (VerticalRotation :type "Float (double-precision)"))
  (bind (_relativerotation_roll _relativerotation_pitch) (`KismetMathLibrary.BreakRotator` (`SceneComponent.RelativeRotation` (`self.CameraMesh`))))
  (bind (_relativerotation_roll_2 _relativerotation_pitch_2 _relativerotation_yaw) (`KismetMathLibrary.BreakRotator` (`SceneComponent.RelativeRotation` (`self.RotatorMesh`))))
  (return _relativerotation_yaw (* _relativerotation_pitch -1.0)))

(fn `UserConstructionScript`
  (`parent.UserConstructionScript`)
  (set `self.MeshToOutline` (`|MakeArray` (`self.ArmMesh`) (`self.CameraMesh`) :!type "MeshComponent Object Reference")))