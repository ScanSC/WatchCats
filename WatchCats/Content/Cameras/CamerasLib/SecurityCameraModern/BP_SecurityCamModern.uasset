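; BP_SecurityCamModern is the modern security camera Blueprint, which adds cursor hover highlighting to the camera.
; When the cursor enters DetectionBox, it calls HighlightObject on the Cyl and Sphere meshes with a modern-camera outline material instance.
; When the cursor leaves, it makes the same call with no material set.
; The construction script only calls its parent, and the other event nodes are disabled.
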(event `self.DetectionBox.OnBeginCursorOver`
  (params (TouchedComponent :type "PrimitiveComponent Object Reference"))
  (`self.Highlight Object` (`|MakeArray` (`self.Cyl`) (`self.Sphere`) :!type "MeshComponent Object Reference") "/Game/Cameras/Materials/M_Outline_ModernCamera_Inst.M_Outline_ModernCamera_Inst"))

(event `self.DetectionBox.OnEndCursorOver`
  (params (TouchedComponent :type "PrimitiveComponent Object Reference"))
  (`self.Highlight Object` (`|MakeArray` (`self.Cyl`) (`self.Sphere`) :!type "MeshComponent Object Reference")))

(fn `UserConstructionScript`
  (`parent.UserConstructionScript`))