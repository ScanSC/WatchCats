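; Base pawn for hackable cameras that the player looks through, with constrained rotation, zoom-scaled look speed, FOV zoom, HUD and pause menu.
; Cursor hover on a camera's DetectionBox outlines it and registers it in the GameInstance.
; Holding input runs a timeline driving that camera's hack bar and a post-process shader, then swaps possession behind a transition widget.
; The initially possessed camera also creates shared alert, dialog and popup widgets.
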(event `self.ReceiveBeginPlay`
  (`|ExecutionSequence`
    (:`then_0`
      ;[1 1 1] BeginPlay : Get controller
      (bind _asplayer_controller (cast `PlayerController` (`self.GetController`)))
      (bind _returnvalue (pcsubsystem `EnhancedInputLocalPlayerSubsystem` _asplayer_controller))
      (`/Engine/EditorBlueprintResources/StandardMacros.IsValid` _returnvalue
        (:`Is Valid`
          (`EnhancedInputSubsystemInterface.AddMappingContext` _returnvalue "/Game/Cameras/Inputs/CameraInputs.CameraInputs" 0 (struct))
          (bind _returnvalue_2 (`EnhancedInputSubsystemInterface.GetUserSettings` _returnvalue))
          (if (not (`EnhancedInputUserSettings.IsMappingContextRegistered` _returnvalue_2 "/Game/Cameras/Inputs/CameraInputs.CameraInputs"))
            (`EnhancedInputUserSettings.RegisterInputMappingContext` _returnvalue_2 null)))))
    (:`then_1`
      ;[1 1 1] BeginPlay : Set HUD
      (bind _returnvalue_3 (`|CreateWidget` (`self.HUDClass`)))
      (bind _output_get (set `self.HUD` _returnvalue_3))
      (set `Widget.Visibility` "HitTestInvisible" _output_get)
      (`/Game/Cameras/HUD/WBP_Camera.SetupHud` _output_get self))
    (:`then_2`
      ;[1 1 1] Get GameInstance
      (bind _asbp_game_instance (cast `/Game/BP_GameInstance` (`GameplayStatics.GetGameInstance`)))
      (set `self.Game Instance` _asbp_game_instance))
    (:`then_3`
      ;[1 1 1] If default possess
      (if (== self (`GameplayStatics.GetPlayerPawn` 0))
        (`PrimitiveComponent.SetCollisionEnabled` (`self.DetectionBox`) "NoCollision")
        (`UserWidget.AddToViewport` (`self.HUD`) 0)
        (`self.DefaultPossess`)))
    (:`then_4`
      (`self.SetupTransitionShader`))))

(event `EnhancedInput|/Game/Cameras/Inputs/InputActions/IA_Look`
  (params (ActionValue :type "Vector2D Structure") (ElapsedSeconds :type "Float (double-precision)") (TriggeredSeconds :type "Float (double-precision)") (InputAction :type "InputAction Object Reference" :default "/Game/Cameras/Inputs/InputActions/IA_Look.IA_Look"))
  (bind _rotatingsfx (`self.RotatingSfx`))
  ;[1 1 1] Look Input Event: rotate camera
  (:`Triggered`
    (bind (_xout _yout) (`self.GetRotationModifier` ActionValue_X ActionValue_Y))
    (bind (_newhorizontalrotation _newverticalrotation) (`self.ContraintViewModifiers` _xout _yout))
    (`SceneComponent.K2_SetRelativeRotation` (`self.Camera`) (`KismetMathLibrary.MakeRotator` 0.0 _newverticalrotation _newhorizontalrotation) true false)
    (`/Engine/EditorBlueprintResources/StandardMacros.IsValid` _rotatingsfx
      (:`Is Valid`
        (if (not (`AudioComponent.IsPlaying` _rotatingsfx))
          (`AudioComponent.Play` (`self.RotatingSfx`) 0.0)))
      (:`Is Not Valid`
        (bind _returnvalue (`GameplayStatics.SpawnSound2D` "/Game/Cameras/CamerasLib/Computer/Audio/Sfx_CameraRotation_Cue.Sfx_CameraRotation_Cue" 1.0 1.0 0.0 null))
        (set `self.RotatingSfx` _returnvalue))))
  (:`Completed`
    (`AudioComponent.Stop` (`self.RotatingSfx`))))

(event `Highlight Object`
  (params (`On/Off` :type Boolean))
  (bind _meshtooutline (`self.MeshToOutline`))
  ;[1 1 1] Highlight object
  (if `On/Off`
    (for _array_element _meshtooutline
      (`MeshComponent.SetOverlayMaterial` _array_element "/Game/Cameras/Materials/M_Outline_Inst.M_Outline_Inst"))
    (else
      (for _array_element_2 _meshtooutline
        (`MeshComponent.SetOverlayMaterial` _array_element_2 null)))))

(event `EnhancedInput|/Game/Cameras/Inputs/InputActions/IA_Scroll`
  (params (ActionValue :type "Float (double-precision)") (ElapsedSeconds :type "Float (double-precision)") (TriggeredSeconds :type "Float (double-precision)") (InputAction :type "InputAction Object Reference" :default "/Game/Cameras/Inputs/InputActions/IA_Scroll.IA_Scroll"))
  ;[1 1 1] Zoom
  (:`Triggered`
    (bind _camera (`self.GetCamera`))
    (`self.UpdateZoom` _camera ActionValue)))

(event `EnhancedInput|/Game/Cameras/Inputs/InputActions/IA_Hold`
  (params (ActionValue :type Boolean) (ElapsedSeconds :type "Float (double-precision)") (TriggeredSeconds :type "Float (double-precision)") (InputAction :type "InputAction Object Reference" :default "/Game/Cameras/Inputs/InputActions/IA_Hold.IA_Hold"))
  (bind _overedcamera (`/Game/BP_GameInstance.OveredCamera` (`self.Game Instance`)))
  ;[1 1 1] Hack camera
  (:`Triggered`
    (`/Engine/EditorBlueprintResources/StandardMacros.IsValid` _overedcamera
      (:`Is Not Valid`
        (`self.StopHacking` :!label _label
          (:`ExecOut`
            (bind (_direction _alpha) (`Timeline|HackingTimeline` :!via `Stop` :!label _label_2)
              (:`Update`
                (bind _returnvalue (`KismetMathLibrary.Lerp` 0.0 100.0 _alpha))
                (`self.SetHackingPercentage` _overedcamera _returnvalue)
                (`self.SetTransitionShaderValue` (- 1.0 (/ _returnvalue 100.0))))
              (:`Finished`
                (`self.StopHacking`
                  (:`ExecOut`
                    (`self.SwapCamera` _overedcamera))))))))))
  (:`Started`
    (`/Engine/EditorBlueprintResources/StandardMacros.IsValid` _overedcamera
      (:`Is Valid`
        (`self.StartHacking`
          (:`ExecOut`
            (goto _label_2 :!via `PlayFromStart`))))))
  (:`Canceled`
    (goto _label))
  (:`Completed`
    (goto _label)))

(event `SwapCamera`
  (params (Camera :type "/Game/Cameras/BP_AbstractCamera Object Reference"))
  ;[1 1 1] Swap Camera
  (`|ExecutionSequence`
    (:`then_0`
      (bind _returnvalue (`|CreateWidget` "/Game/Cameras/HUD/WBP_Transition.WBP_Transition_C"))
      (`UserWidget.AddToViewport` _returnvalue 0))
    (:`then_1`
      (bind _returnvalue_2 (`GameplayStatics.SpawnSound2D` "/Game/Cameras/Audios/Hacking_Transition_Audio.Hacking_Transition_Audio" 1.0 1.0 0.5 null))))
  (`KismetSystemLibrary.Delay` 0.3)
  (`|ExecutionSequence`
    (:`then_0`
      (`Widget.RemoveFromParent` _returnvalue)
      (`self.UnpossessCamera`)
      (`self.PossessCamera` Camera))
    (:`then_1`
      (`AudioComponent.Stop` _returnvalue_2))))

(event `EnhancedInput|/Game/Cameras/Inputs/InputActions/IA_PauseMenu`
  (params (ActionValue :type Boolean) (ElapsedSeconds :type "Float (double-precision)") (TriggeredSeconds :type "Float (double-precision)") (InputAction :type "InputAction Object Reference" :default "/Game/Cameras/Inputs/InputActions/IA_PauseMenu.IA_PauseMenu"))
  (bind _returnvalue (`GameplayStatics.GetPlayerController` 0))
  ;[1 1 1] Pause menu
  (:`Triggered`
    (if (not (`self.IsPaused?`))
      (set `self.IsPaused?` true)
      (bind _returnvalue_2 (`|CreateWidget` "/Game/UI/WBP_PauseMenu.WBP_PauseMenu_C" _returnvalue))
      (bind _output_get (set `self.Pause Menu` _returnvalue_2))
      (`UserWidget.AddToViewport` _output_get 0)
      (`WidgetBlueprintLibrary.SetInputMode_GameAndUIEx` _returnvalue (`self.Pause Menu`))
      (set `PlayerController.bShowMouseCursor` true (`GameplayStatics.GetPlayerController` 0))
      (`GameplayStatics.SetGamePaused` true)
      (else
        (set `self.IsPaused?` false)
        (`Widget.RemoveFromParent` (`self.Pause Menu`))
        (`GameplayStatics.SetGamePaused` false)
        (`WidgetBlueprintLibrary.SetInputMode_GameAndUIEx` _returnvalue null)))))

(event `self.DetectionBox.OnBeginCursorOver`
  (params (TouchedComponent :type "PrimitiveComponent Object Reference"))
  (bind _game_instance (`self.Game Instance`))
  ;[1 1 1] On camera overed
  (bind _output_get (set `/Game/BP_GameInstance.OveredCamera` self _game_instance))
  (set `/Game/BP_GameInstance.LastOveredCamera` _output_get _game_instance)
  (`self.Highlight Object` true))

(event `self.DetectionBox.OnEndCursorOver`
  (params (TouchedComponent :type "PrimitiveComponent Object Reference"))
  (bind _overedcamera (`/Game/BP_GameInstance.OveredCamera` (`self.Game Instance`)))
  ;[1 1 1] On camera unovered
  (`/Engine/EditorBlueprintResources/StandardMacros.IsValid` _overedcamera
    (:`Is Valid`
      (if (== self _overedcamera)
        (set `/Game/BP_GameInstance.OveredCamera` null (`self.Game Instance`) :!label _label)
        (`self.Highlight Object` false)))
    (:`Is Not Valid`
      (goto _label))))

(fn `ContraintViewModifiers`
  (params (HorizontalModifier :type "Float (double-precision)") (VerticalModifier :type "Float (double-precision)"))
  (returns (NewHorizontalRotation :type "Float (double-precision)") (NewVerticalRotation :type "Float (double-precision)"))
  (locals (NewLocalVar :type "Rotator Structure" :default (struct)))
  (bind (_viewconstraints_ishorizontalconstrained _viewconstraints_horizontalmin _viewconstraints_horizontalmax _viewconstraints_isverticalconstrained _viewconstraints_verticalmin _viewconstraints_verticalmax) (break `/Game/Cameras/Struct_ViewConstraints` (`self.ViewConstraints`)))
  (bind (_viewconstraints_ishorizontalconstrained_2 _viewconstraints_horizontalmin_2 _viewconstraints_horizontalmax_2) (break `/Game/Cameras/Struct_ViewConstraints` (`self.ViewConstraints`)))
  (bind (_horizontalrotation _verticalrotation) (`self.GetCameraRotation`))
  (bind _returnvalue (+ HorizontalModifier _horizontalrotation))
  (bind _returnvalue_2 (+ _verticalrotation VerticalModifier))
  (return (select `bool` _viewconstraints_ishorizontalconstrained_2 :`false` _returnvalue :`true` (`KismetMathLibrary.FClamp` _returnvalue (`KismetMathLibrary.Conv_IntToDouble` _viewconstraints_horizontalmin_2) (`KismetMathLibrary.Conv_IntToDouble` _viewconstraints_horizontalmax_2))) (select `bool` _viewconstraints_isverticalconstrained :`false` _returnvalue_2 :`true` (`KismetMathLibrary.FClamp` _returnvalue_2 (`KismetMathLibrary.Conv_IntToDouble` _viewconstraints_verticalmin) (`KismetMathLibrary.Conv_IntToDouble` _viewconstraints_verticalmax)))))

(fn `DefaultPossess`
  (bind _returnvalue (`|CreateWidget` "/Game/UI/WBP_AlertScreenOverlay.WBP_AlertScreenOverlay_C"))
  (set `/Game/BP_GameInstance.AlertScreen` _returnvalue (`self.Game Instance`))
  (bind _returnvalue_2 (`|CreateWidget` "/Game/Text/WBP_Dialog_Box.WBP_Dialog_Box_C"))
  (set `/Game/BP_GameInstance.DialogBox` _returnvalue_2 (`self.Game Instance`))
  (bind _returnvalue_3 (`|CreateWidget` "/Game/Text/WBP_Popup_Text.WBP_Popup_Text_C"))
  (set `/Game/BP_GameInstance.PopupText` _returnvalue_3 (`self.Game Instance`))
  (bind _returnvalue_4 (`|CreateWidget` "/Game/Text/WBP_Popup_Alert.WBP_Popup_Alert_C"))
  (set `/Game/BP_GameInstance.PopupAlert` _returnvalue_4 (`self.Game Instance`)))

(fn `GetCamera`
  (returns (Camera :type "CameraComponent Object Reference"))
  (return (`self.Camera`)))

(fn `GetCameraRotation`
  (returns (HorizontalRotation :type "Float (double-precision)") (VerticalRotation :type "Float (double-precision)"))
  (bind (_relativerotation_roll _relativerotation_pitch _relativerotation_yaw) (`KismetMathLibrary.BreakRotator` (`SceneComponent.RelativeRotation` (`self.Camera`))))
  (return _relativerotation_yaw _relativerotation_pitch))

(fn `GetInteractMessage`
  (returns (Message :type Text))
  (return (`self.Name`)))

(fn `GetRotationModifier`
  (params (Xin :type "Float (double-precision)") (Yin :type "Float (double-precision)"))
  (returns (Xout :type "Float (double-precision)") (Yout :type "Float (double-precision)"))
  (bind _rotationspeedmodifier (`self.RotationSpeedModifier`))
  (bind (_zoom_max _zoom_value) (break `/Game/Cameras/Struct_Zoom` (`self.Zoom`)))
  (return (/ (* Xin _rotationspeedmodifier) _zoom_value) (/ (* Yin _rotationspeedmodifier) _zoom_value)))

(fn `PossessCamera`
  (`Controller.Possess` (`GameplayStatics.GetPlayerController` 0) self)
  (`PrimitiveComponent.SetCollisionEnabled` (`self.DetectionBox`) "NoCollision")
  (`UserWidget.AddToViewport` (`self.HUD`) 0))

(fn `SetHackingPercentage`
  (params (Percentage :type "Float (double-precision)"))
  (bind _output_get (set `self.HackingPercentage` Percentage))
  (bind _aswbp_hold (cast `/Game/Cameras/HUD/WBP_Hold` (`WidgetComponent.GetUserWidgetObject` (`self.HackingBar`))))
  (`/Game/Cameras/HUD/WBP_Hold.SetPercentage` _aswbp_hold _output_get))

(fn `SetTransitionShaderValue`
  (params (Transition :type "Float (double-precision)" :default 1.0))
  (bind _transitionshader (`self.TransitionShader`))
  (`/Engine/EditorBlueprintResources/StandardMacros.IsValid` _transitionshader
    (:`Is Valid`
      (`MaterialInstanceDynamic.SetScalarParameterValue` _transitionshader "Transition" Transition))))

(fn `SetupTransitionShader`
  (bind _returnvalue (`KismetMaterialLibrary.CreateDynamicMaterialInstance` "/Game/Materials/PostProcess/M_PostProcessHacking.M_PostProcessHacking"))
  (bind _camera (`self.GetCamera`))
  (bind _output_get (set `self.TransitionShader` _returnvalue))
  (`KismetArrayLibrary.Array_Add` (`.Array` (break `WeightedBlendables` (`.WeightedBlendables` (break `PostProcessSettings` (`CameraComponent.PostProcessSettings` _camera))))) (make `WeightedBlendable` 1.0 _output_get))
  (`self.SetTransitionShaderValue` 1.0))

(fn `UnpossessCamera`
  (`Widget.RemoveFromParent` (`self.HUD`))
  (`PrimitiveComponent.SetCollisionEnabled` (`self.DetectionBox`) "QueryOnly"))

(fn `UpdateZoom`
  (params (Camera :type "CameraComponent Object Reference") (ActionValue :type "Float (double-precision)"))
  (bind (_zoom_max _zoom_value) (break `/Game/Cameras/Struct_Zoom` (`self.Zoom`)))
  (bind _output_get (set `self.Zoom` (make `/Game/Cameras/Struct_Zoom` _zoom_max (`KismetMathLibrary.FClamp` (+ _zoom_value (/ ActionValue 10.0)) 1.0 _zoom_max))))
  (`CameraComponent.SetFieldOfView` Camera (- 90.0 (* (- (`.Value_7_59884E6D4AC6A4964BFC2893D8ED9398` (break `/Game/Cameras/Struct_Zoom` _output_get)) 1.0) 30.0)))
  (`/Game/Cameras/HUD/WBP_Camera.SetZoomValue` (`self.HUD`) (`.Value_7_59884E6D4AC6A4964BFC2893D8ED9398` (break `/Game/Cameras/Struct_Zoom` _output_get))))

(fn `UserConstructionScript`)