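; BP_Computer is a clickable computer actor that opens a hacking popup.
; BeginPlay caches the player controller and game instance and pre-creates the WBP_Computer_Popup widget.
; Cursor events on its Cube track HoveredComputer in the game instance; clicking registers it as HackedComputer and shows the popup if that slot is free.
; Interact prompts and already-hacking feedback are temporary PrintString placeholders.
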(event `self.ReceiveBeginPlay`
  (`|ExecutionSequence`
    (:`then_0`
      ;[1 1 1] Get plqyer reference
      (bind _asbp_player_controller (cast `/Game/Cameras/BP_PlayerController` (`GameplayStatics.GetPlayerController` 0)))
      (set `self.Player Ref` _asbp_player_controller))
    (:`then_1`
      ;[1 1 1] get game instance
      (bind _asbp_game_instance (cast `/Game/BP_GameInstance` (`GameplayStatics.GetGameInstance`)))
      (set `self.Game Instance` _asbp_game_instance))
    (:`then_2`
      ;[1 1 1] Initialize interface
      (bind _returnvalue (`|CreateWidget` "/Game/Computer/HUD/WBP_Computer_Popup.WBP_Computer_Popup_C"))
      (set `self.HUDWidget` _returnvalue))))

(event `self.Cube.OnClicked`
  (params (TouchedComponent :type "PrimitiveComponent Object Reference") (ButtonPressed :type "Key Structure"))
  ;[1 1 1] (On Clicked) get window to pirate the computer
  (if (== (`/Game/BP_GameInstance.HackedComputer` (`self.Game Instance`)) null)
    (set `/Game/BP_GameInstance.HackedComputer` self (`self.Game Instance`))
    (`UserWidget.AddToViewport` (`self.HUDWidget`) 0)
    (else
      ;;[1 0 0] TMP (already hacking a PC)
      (`KismetSystemLibrary.PrintString` "Hello"))))

(event `self.Cube.OnBeginCursorOver`
  (params (TouchedComponent :type "PrimitiveComponent Object Reference"))
  ;[1 1 1] (On Over) set the hovered computer value in game instance
  (set `/Game/BP_GameInstance.HoveredComputer` self (`self.Game Instance`))
  ;;[1 0 0] TMP (show interact message)
  (`KismetSystemLibrary.PrintString` "show interact message"))

(event `self.Cube.OnEndCursorOver`
  (params (TouchedComponent :type "PrimitiveComponent Object Reference"))
  ;[1 1 1] (On leave) unset game instance hovered value
  (`/Engine/EditorBlueprintResources/StandardMacros.IsValid` null
    (:`Is Valid`
      (if (== self (`/Game/BP_GameInstance.HoveredComputer` (`self.Game Instance`)))
        (set `/Game/BP_GameInstance.HoveredComputer` null (`self.Game Instance`) :!label _label)
        ;;[1 0 0] TMP (remove interact message)
        (`KismetSystemLibrary.PrintString` "remove hud")))
    (:`Is Not Valid`
      (goto _label))))

(fn `UserConstructionScript`)