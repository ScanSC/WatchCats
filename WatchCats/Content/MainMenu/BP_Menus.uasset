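; BP_Menus is a main menu actor that hosts a WBP_Menus widget and moves the player's view between linked menu actors.
; BeginPlay adds the CameraInputs mapping context and, only if it is not yet registered, registers it and binds the widget's transition event.
; That event picks a LinkedMenus entry by index, swaps collision from this actor to the target and eases the view target across.
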(event `self.ReceiveBeginPlay`
  (bind _returnvalue (pcsubsystem `EnhancedInputLocalPlayerSubsystem` (`GameplayStatics.GetPlayerController` 0)))
  (bind _returnvalue_2 (`EnhancedInputSubsystemInterface.GetUserSettings` _returnvalue))
  (`/Engine/EditorBlueprintResources/StandardMacros.IsValid` _returnvalue
    (:`Is Valid`
      (`EnhancedInputSubsystemInterface.AddMappingContext` _returnvalue "/Game/Devices/HackableDevices/Cameras/Inputs/CameraInputs.CameraInputs" 0 (struct))
      (if (not (`EnhancedInputUserSettings.IsMappingContextRegistered` _returnvalue_2 "/Game/Devices/HackableDevices/Cameras/Inputs/CameraInputs.CameraInputs"))
        (`EnhancedInputUserSettings.RegisterInputMappingContext` _returnvalue_2 "/Game/Devices/HackableDevices/Cameras/Inputs/CameraInputs.CameraInputs")
        (bind _aswbp_menus (cast `/Game/UI/WBP_Menus` (`WidgetComponent.GetUserWidgetObject` (`self.Widget`))))
        (add `/Game/UI/WBP_Menus.TransitionToLinkedMenu` _aswbp_menus (delegate `TransitionBewteenMenus`))))))

(event `TransitionBewteenMenus`
  (params (Index :type Integer))
  (bind _linkedmenus (`self.LinkedMenus`))
  (if (`KismetArrayLibrary.Array_IsValidIndex` _linkedmenus Index)
    (`self.Transition` (`|GetArrayItem` _linkedmenus Index))))

(event `Transition`
  (params (NewMenu :type "/Game/MainMenu/BP_Menus Object Reference"))
  (`self.SetActorEnableCollision` false)
  (`self.SetActorEnableCollision` NewMenu true)
  (`PlayerController.SetViewTargetWithBlend` (`GameplayStatics.GetPlayerController` 0) NewMenu 2.0 "VTBlend_EaseInOut" 2.0 false))

(fn `UserConstructionScript`)