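; BP_ElevatorDoor is a connected-device Blueprint for a two-panel sliding elevator door.
; Activate calls the parent implementation, then runs Open or Close based on IsActive, and each of those events also sets that flag.
; A single timeline lerps both panels' relative X positions in mirror image, playing from the start to open and reversing to close.
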(event `Open`
  (set `self.isActive` true)
  (bind (_direction _alpha) (`Timeline|DoorTimeline` :!via `PlayFromStart` :!label _label)
    (:`Update`
      (bind _returnvalue (`KismetMathLibrary.Lerp` 125.0 325.0 _alpha))
      (`SceneComponent.K2_SetRelativeLocation` (`self.DoorR`) (`KismetMathLibrary.MakeVector` _returnvalue 0.0 300.0) false false)
      (`SceneComponent.K2_SetRelativeLocation` (`self.DoorL`) (`KismetMathLibrary.MakeVector` (* _returnvalue -1.0) 0.0 300.0) false false))))

(event `Close`
  (set `self.isActive` false)
  (goto _label :!via `Reverse`))

(fn `Activate`
  (`parent.Activate`)
  (if (`self.isActive`)
    (`self.Open`)
    (else
      (`self.Close`))))

(fn `UserConstructionScript`
  (`parent.UserConstructionScript`))