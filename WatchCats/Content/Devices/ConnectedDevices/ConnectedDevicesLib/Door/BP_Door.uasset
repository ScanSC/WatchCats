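; Sliding door in the connected devices library that opens and closes according to its IsActive state.
; Activate runs the parent logic, then calls Open or Close, which set the state and fire the door events; BeginPlayNext applies the initial state.
; A timeline slides the box along relative X, played with a 2D sound to open and reversed to close.
; The construction script labels two door marks with the device's name and color.
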(event `BeginPlayNext_1`
  (`|ExecutionSequence`
    (:`then_0`
      (if (`self.isActive`)
        (`self.Open` null)
        (else
          (`self.Close`))))))

(event `OpenDoor`
  (params (SlideAudio :type "SoundBase Object Reference"))
  (bind _box (`self.Box`))
  (bind (_relativelocation_x _relativelocation_y _relativelocation_z) (`KismetMathLibrary.BreakVector` (`SceneComponent.RelativeLocation` _box)))
  (`GameplayStatics.PlaySound2D` SlideAudio 1.0 1.0 0.0 null null)
  (bind (_direction _alpha) (`Timeline|OpeningTimeline` :!label _label)
    (:`Update`
      (`SceneComponent.K2_SetRelativeLocation` _box (`KismetMathLibrary.MakeVector` (`KismetMathLibrary.Lerp` 0.0 -250.0 _alpha) _relativelocation_y _relativelocation_z) false false))))

(event `CloseDoor`
  (goto _label :!via `Reverse`))

(fn `Activate`
  (`parent.Activate`)
  (if (`self.isActive`)
    (`self.Open` "/Game/Devices/ConnectedDevices/ConnectedDevicesLib/SFX/SlidingDoor.SlidingDoor")
    (else
      (`self.Close`))))

(fn `Close`
  (set `self.isActive` false)
  (`self.CloseDoor`))

(fn `Open`
  (params (Sound :type "SoundBase Object Reference"))
  (set `self.isActive` true)
  (`self.OpenDoor` Sound))

(fn `UserConstructionScript`
  (bind _color (`self.Color`))
  (bind _name (`self.Name`))
  (`|ExecutionSequence`
    (:`then_0`
      (`TextRenderComponent.K2_SetText` (`self.DoorMark1`) _name)
      (`TextRenderComponent.K2_SetText` (`self.DoorMark2`) _name)
      (`TextRenderComponent.SetTextRenderColor` (`self.DoorMark1`) _color)
      (`TextRenderComponent.SetTextRenderColor` (`self.DoorMark2`) _color))))