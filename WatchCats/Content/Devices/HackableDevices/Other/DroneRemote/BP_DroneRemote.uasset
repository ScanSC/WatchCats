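; Hackable remote that pilots a linked drone through two interactive widget pads, one for movement and one for the camera.
; Both pads receive a reference to the remote, whose functions forward direction, rotation, zoom and camera reset to the drone.
; It starts powered off, and each hack toggles power, swapping the screen material, showing or hiding the drone's HUD, and opening or closing the pads with their collision and a hologram sound.
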(event `self.ReceiveBeginPlay`
  (`parent.ReceiveBeginPlay`)
  (`|ExecutionSequence`
    (:`then_0`
      (`WidgetComponent.SetWidget` (`self.DroneHUD`) (`/Game/Devices/HackableDevices/Cameras/BP_AbstractCamera.HUD` (`self.Drone`))))
    (:`then_1`
      ;[1 1 1] Setup Outline
      (`KismetArrayLibrary.Array_Add` (`self.MeshToOutline`) (`self.Remote`)))
    (:`then_2`
      ;[1 1 1] Give itself to Controls Widgets
      (bind _aswbp_drone_controls (cast `/Game/Devices/HackableDevices/Other/DroneRemote/WBP_DroneControls` (`WidgetComponent.GetWidget` (`self.ControlsWidget`))))
      (set `/Game/Devices/HackableDevices/Other/DroneRemote/WBP_DroneControls.Parent` self _aswbp_drone_controls)
      (bind _aswbp_drone_camera_controls (cast `/Game/Devices/HackableDevices/Other/DroneRemote/WBP_DroneCameraControls` (`WidgetComponent.GetWidget` (`self.CameraControlsWidget`))))
      (set `/Game/Devices/HackableDevices/Other/DroneRemote/WBP_DroneCameraControls.Parent` self _aswbp_drone_camera_controls)
      ;[1 1 1] Power Off
      (`self.PowerOn/Off` false))))

(fn `ChangeDroneCameraDirection`
  (params (Direction :type "Vector2D Structure"))
  (set `/Game/Devices/HackableDevices/Cameras/CamerasLib/Drone/BP_Drone.CameraDirection` (`KismetMathLibrary.MakeVector2D` Direction_Y Direction_X) (`self.Drone`)))

(fn `ChangeDroneDirections`
  (params (Direction :type "Vector Structure"))
  (set `/Game/Devices/HackableDevices/Cameras/CamerasLib/Drone/BP_Drone.Direction` Direction (`self.Drone`)))

(fn `ChangeDroneRotation`
  (params (Rotation :type Integer))
  (set `/Game/Devices/HackableDevices/Cameras/CamerasLib/Drone/BP_Drone.RotationMouvement` Rotation (`self.Drone`)))

(fn `ChangeDroneZoom`
  (params (Modifier :type "Float (double-precision)"))
  (set `/Game/Devices/HackableDevices/Cameras/CamerasLib/Drone/BP_Drone.ZoomModifier` Modifier (`self.Drone`)))

(fn `Hacked`
  (`parent.Hacked`)
  (if (`self.IsOn`)
    (`self.PowerOn/Off` false)
    (else
      (`self.PowerOn/Off` true))))

(fn `ResetDroneCamera`
  (`/Game/Devices/HackableDevices/Cameras/CamerasLib/Drone/BP_Drone.ResetCamera` (`self.Drone`)))

(fn `UserConstructionScript`)