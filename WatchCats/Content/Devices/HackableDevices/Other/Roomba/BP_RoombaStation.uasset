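; BP_RoombaStation is a hackable docking station for the Roomba that gives access to a map once a Roomba has docked.
; When a BP_Roomba overlaps its Box, the station deactivates it, flags itself as connected and turns its LED bright green.
; The map widget is created at BeginPlay and only added to the viewport when the station is hacked while that connected flag is set.
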(event `self.ReceiveBeginPlay`
  (`parent.ReceiveBeginPlay`)
  (bind _returnvalue (`|CreateWidget` "/Game/Devices/HackableDevices/Other/Roomba/WBP_Map.WBP_Map_C"))
  (set `self.MapWidget` _returnvalue))

(event `self.Box.OnComponentBeginOverlap`
  (params (OverlappedComponent :type "PrimitiveComponent Object Reference") (OtherActor :type "Actor Object Reference") (OtherComp :type "PrimitiveComponent Object Reference") (OtherBodyIndex :type Integer) (bFromSweep :type Boolean) (SweepResult :type "HitResult Structure (by ref)"))
  (bind _asbp_roomba (cast `/Game/Devices/HackableDevices/Other/Roomba/BP_Roomba` OtherActor))
  (`/Game/Devices/HackableDevices/Other/Roomba/BP_Roomba.Deactivate` _asbp_roomba)
  (set `self.IsConnectedToRoomba` true)
  (`PrimitiveComponent.SetMaterial` (`self.Led`) 0 "/Game/Materials/Mat_GreenBright.Mat_GreenBright"))

(fn `Hacked`
  (`parent.Hacked`)
  (if (`self.IsConnectedToRoomba`)
    (`UserWidget.AddToViewport` (`self.MapWidget`) 0)))

(fn `UserConstructionScript`
  (`parent.UserConstructionScript`))