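; BP_Roomba is a hackable Roomba device whose hack toggles between autonomous mode and player control.
; Taking or leaving control flips IsAutonomous and shows or hides the WBP_RoombaControls pad and controlled indicator, with a hologram sound.
; Tick sweeps it along its local Direction times Speed and yaws it by RotationMovement, without delta-time scaling.
; No autonomous steering logic appears in these graphs.
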(event `self.ReceiveBeginPlay`
  (`parent.ReceiveBeginPlay`)
  (`|ExecutionSequence`
    (:`then_0`
      (bind _returnvalue (`|CreateWidget` "/Game/Devices/HackableDevices/Other/Roomba/WBP_RoombaControls.WBP_RoombaControls_C"))
      (bind _output_get (set `self.ControlWidget` _returnvalue))
      (set `/Game/Devices/HackableDevices/Other/Roomba/WBP_RoombaControls.Parent` self _output_get))
    (:`then_1`
      (`self.HideControls` true))))

(event `self.ReceiveTick`
  (params (DeltaSeconds :type "Float (single-precision)"))
  (`self.K2_SetActorLocation` (+ (`KismetMathLibrary.GreaterGreater_VectorRotator` (* (`self.Direction`) (`self.Speed`)) (`self.K2_GetActorRotation`)) (`self.K2_GetActorLocation`)) true)
  (`self.K2_AddActorWorldRotation` (`KismetMathLibrary.MakeRotator` 0.0 0.0 (`KismetMathLibrary.Conv_IntToDouble` (`self.RotationMovement`))) true))

(fn `Hacked`
  (`parent.Hacked`)
  (if (`self.isAutonomous`)
    (`self.TakeControl`)
    (else
      (`self.LeaveControl`))))

(fn `LeaveControl`
  (`self.HideControls` false
    (:`Out`
      (set `self.isAutonomous` true))))

(fn `TakeControl`
  (`self.ShowControls` false
    (:`Out`
      (set `self.isAutonomous` false))))

(fn `UserConstructionScript`
  (`parent.UserConstructionScript`))