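; BP_Codepad is a hackable keypad device that gates activation of a connected device behind a code.
; Hacking it toggles a WBP_Codepad widget component, or activates the device directly once unlocked; the widget hides when another device is hacked.
; SubmitCode plays a sound and, on a match, unlocks and activates the device.
; The connected device's OnActivation event also unlocks the pad and updates its LED material.
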(event `self.ReceiveBeginPlay`
  (`parent.ReceiveBeginPlay`)
  (`|ExecutionSequence`
    (:`then_0`
      ;[1 1 1] Listen Connected Device "OnActivation" Event
      (add `/Game/Devices/ConnectedDevices/BP_AbstractConnectedDevice.OnActivation` (`self.ConnectedDevice`) (delegate `OnActivation_Event`)))
    (:`then_1`
      ;[1 1 1] Listen Game Instance "OnHackedDevice" Event
      (add `/Game/BP_GameInstance.OnHackedDevice` (`self.Game Instance`) (delegate `HideIfNotHacked`)))
    (:`then_2`
      ;[1 1 1] Setup Outline
      (`KismetArrayLibrary.Array_Add` (`self.MeshToOutline`) (`self.Mesh`)))
    (:`then_3`
      ;[1 1 1] Give itself to Codepad Widget
      (bind _aswbp_codepad (cast `/Game/Devices/HackableDevices/Other/Codepad/WBP_Codepad` (`WidgetComponent.GetWidget` (`self.CodepadWidget`))))
      (set `/Game/Devices/HackableDevices/Other/Codepad/WBP_Codepad.Parent` self _aswbp_codepad)
      ;[1 1 1] Hide widget
      (`self.HideCodepad`))))

(event `OnActivation_Event`
  ;[1 1 1] Listen Connected Device "OnActivation" Event
  (`self.Update Leds`)
  (set `self.isUnlocked` true))

(event `HideIfNotHacked`
  ;[1 1 1] Listen Game Instance "OnHackedDevice" Event
  (if (and (!= (`/Game/BP_GameInstance.HackedDevice` (`self.Game Instance`)) self) (`self.IsWidgetShowed`))
    (`self.HideCodepad`)))

(fn `CloseCodepad`
  (`self.HideCodepad`))

(fn `Hacked`
  (`parent.Hacked`)
  (if (`self.isUnlocked`)
    (`/Game/Devices/ConnectedDevices/BP_AbstractConnectedDevice.Activate` (`self.ConnectedDevice`))
    (elif (`self.IsWidgetShowed`)
      (`self.HideCodepad`)
      (else
        (`self.ShowCodepad`)))))

(fn `SubmitCode`
  (params (Code :type String))
  (returns (Success :type Boolean))
  (bind _returnvalue (`SceneComponent.K2_GetComponentLocation` (`self.DefaultSceneRoot`)))
  (if (`KismetStringLibrary.EqualEqual_StrStr` Code (`self.Code`))
    (`GameplayStatics.PlaySoundAtLocation` "/Game/Devices/HackableDevices/Cameras/CamerasLib/Computer/Audio/Sfx_TerminalOut.Sfx_TerminalOut" _returnvalue (struct) 1.0 1.0 0.0 null null null null)
    (`/Game/Devices/ConnectedDevices/BP_AbstractConnectedDevice.Activate` (`self.ConnectedDevice`))
    (set `self.isUnlocked` true)
    (return true)
    (else
      (`GameplayStatics.PlaySoundAtLocation` "/Game/Devices/HackableDevices/Cameras/CamerasLib/Computer/Audio/Sfx_TerminalIn.Sfx_TerminalIn" _returnvalue (struct) 1.0 1.0 0.0 null null null null)
      (return false))))

(fn `Update Leds`
  (bind _mesh (`self.Mesh`))
  (if (`/Game/Devices/ConnectedDevices/BP_AbstractConnectedDevice.isActive` (`self.ConnectedDevice`))
    (`PrimitiveComponent.SetMaterial` _mesh 5 "/Game/Materials/Mat_GreenBright.Mat_GreenBright")
    (else
      (`PrimitiveComponent.SetMaterial` _mesh 5 "/Game/Materials/Mat_RedBright.Mat_RedBright"))))

(fn `UserConstructionScript`
  (`parent.UserConstructionScript`))