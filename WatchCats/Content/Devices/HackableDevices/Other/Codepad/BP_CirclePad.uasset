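; BP_CirclePad is a codepad-style hackable device that responds to the outcome of a minigame.
; On success it plays a terminal sound at its location, activates its connected device and marks itself unlocked.
; On failure it only plays a different terminal sound.
; BeginPlay and construction defer entirely to the parent class.
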(event `self.ReceiveBeginPlay`
  (`parent.ReceiveBeginPlay`))

(fn `MiniGameOutcome`
  (params (Success :type Boolean))
  (bind _returnvalue (`SceneComponent.K2_GetComponentLocation` (`self.DefaultSceneRoot`)))
  (if Success
    (`GameplayStatics.PlaySoundAtLocation` "/Game/Devices/HackableDevices/Cameras/CamerasLib/Computer/Audio/Sfx_TerminalOut.Sfx_TerminalOut" _returnvalue (struct) 1.0 1.0 0.0 null null null null)
    (`/Game/Devices/ConnectedDevices/BP_AbstractConnectedDevice.Activate` (`self.ConnectedDevice`))
    (set `self.isUnlocked` true)
    (else
      (`GameplayStatics.PlaySoundAtLocation` "/Game/Devices/HackableDevices/Cameras/CamerasLib/Computer/Audio/Sfx_TerminalIn.Sfx_TerminalIn" _returnvalue (struct) 1.0 1.0 0.0 null null null null))))

(fn `UserConstructionScript`
  (`parent.UserConstructionScript`))