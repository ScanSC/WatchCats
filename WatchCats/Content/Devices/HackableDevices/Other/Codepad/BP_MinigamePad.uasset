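; BP_MinigamePad is a hackable codepad device that hosts a minigame and unlocks a connected device when the minigame succeeds.
; On BeginPlay it creates the minigame widget and assigns it to its CodepadWidget component, then runs the parent's BeginPlay.
; MiniGameOutcome plays a terminal sound at the hit box for either result; success also activates the connected device and marks the pad unlocked.
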(event `self.ReceiveBeginPlay`
  (bind _returnvalue (`|CreateWidget` (`self.MinigameWidget`)))
  (`WidgetComponent.SetWidget` (`self.CodepadWidget`) _returnvalue)
  (`parent.ReceiveBeginPlay`))

(fn `MiniGameOutcome`
  (params (Success :type Boolean))
  (bind _returnvalue (`SceneComponent.K2_GetComponentLocation` (`self.HitBox`)))
  (if Success
    (`GameplayStatics.PlaySoundAtLocation` "/Game/Devices/HackableDevices/Cameras/CamerasLib/Computer/Audio/Sfx_TerminalOut.Sfx_TerminalOut" _returnvalue (struct) 1.0 1.0 0.0 null null null null)
    (`/Game/Devices/ConnectedDevices/BP_AbstractConnectedDevice.Activate` (`self.ConnectedDevice`))
    (set `self.isUnlocked` true)
    (else
      (`GameplayStatics.PlaySoundAtLocation` "/Game/Devices/HackableDevices/Cameras/CamerasLib/Computer/Audio/Sfx_TerminalIn.Sfx_TerminalIn" _returnvalue (struct) 1.0 1.0 0.0 null null null null))))

(fn `UserConstructionScript`
  (`parent.UserConstructionScript`))