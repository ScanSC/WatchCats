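; Base hackable security camera pawn that the player possesses and looks through, hopping to another camera by hacking it.
; Possession swaps the HUD and detection box collision, with SwapCamera adding a timed transition widget and sound.
; Enhanced Input drives clamped rotation that slows with zoom, FOV-based zoom with looping-style SFX control, and the pause menu.
; The default-possessed camera also creates the GameInstance's shared alert, dialog and popup widgets.
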(event `EnhancedInput|/Game/Devices/HackableDevices/Cameras/Inputs/InputActions/IA_Look`
  (params (ActionValue :type "Vector2D Structure") (ElapsedSeconds :type "Float (double-precision)") (TriggeredSeconds :type "Float (double-precision)") (InputAction :type "InputAction Object Reference" :default "/Game/Devices/HackableDevices/Cameras/Inputs/InputActions/IA_Look.IA_Look"))
  (bind _rotatingsfx_0 (`self.RotatingSfx_0`))
  ;[1 1 1] Look Input Event: rotate camera
  (:`Triggered`
    (`self.RotateCamera` ActionValue_X ActionValue_Y)
    (`/Engine/EditorBlueprintResources/StandardMacros.IsValid` _rotatingsfx_0
      (:`Is Valid`
        (if (not (`AudioComponent.IsPlaying` _rotatingsfx_0))
          (`AudioComponent.Play` (`self.RotatingSfx_0`) 0.0)))
      (:`Is Not Valid`
        (bind _returnvalue (`GameplayStatics.SpawnSound2D` "/Game/Devices/HackableDevices/Cameras/CamerasLib/Computer/Audio/Sfx_CameraRotation_Cue.Sfx_CameraRotation_Cue" 1.0 1.0 0.0 null))
        (set `self.RotatingSfx_0` _returnvalue))))
  (:`Started`
    (`self.OnLookInput`))
  (:`Completed`
    (`AudioComponent.Stop` (`self.RotatingSfx_0`))))

(event `SwapCamera`
  (params (Camera :type "/Game/Devices/HackableDevices/Cameras/BP_AbstractCamera Object Reference"))
  ;[1 1 1] Swap Camera
  (`|ExecutionSequence`
    (:`then_0`
      (bind _returnvalue (`|CreateWidget` "/Game/Devices/HackableDevices/Cameras/HUD/WBP_Transition.WBP_Transition_C"))
      (`UserWidget.AddToViewport` _returnvalue 0))
    (:`then_1`
      (bind _returnvalue_2 (`GameplayStatics.SpawnSound2D` "/Game/Audio/SFX/Hacking_Transition_Audio.Hacking_Transition_Audio" 1.0 1.0 0.5 null))))
  (`KismetSystemLibrary.Delay` 0.3)
  (`|ExecutionSequence`
    (:`then_0`
      (`Widget.RemoveFromParent` _returnvalue)
      (`self.UnpossessCamera`)
      (`self.PossessCamera` Camera))
    (:`then_1`
      (`AudioComponent.Stop` _returnvalue_2))))

(event `EnhancedInput|/Game/Devices/HackableDevices/Cameras/Inputs/InputActions/IA_PauseMenu`
  (params (ActionValue :type Boolean) (ElapsedSeconds :type "Float (double-precision)") (TriggeredSeconds :type "Float (double-precision)") (InputAction :type "InputAction Object Reference" :default "/Game/Devices/HackableDevices/Cameras/Inputs/InputActions/IA_PauseMenu.IA_PauseMenu"))
  (bind _returnvalue (`GameplayStatics.GetPlayerController` 0))
  ;[1 1 1] Pause menu
  (:`Triggered`
    (if (not (`/Game/Devices/HackableDevices/Cameras/BP_GameModeCamera.isPaused?` (`self.Game Mode Camera`)))
      (set `/Game/Devices/HackableDevices/Cameras/BP_GameModeCamera.isPaused?` true (`self.Game Mode Camera`))
      (bind _returnvalue_2 (`|CreateWidget` "/Game/UI/WBP_PauseMenu.WBP_PauseMenu_C" _returnvalue))
      (bind _output_get (set `self.Pause Menu` _returnvalue_2))
      (`UserWidget.AddToViewport` _output_get 0)
      (`WidgetBlueprintLibrary.SetInputMode_GameAndUIEx` _returnvalue (`self.Pause Menu`))
      (set `PlayerController.bShowMouseCursor` true (`GameplayStatics.GetPlayerController` 0))
      (`GameplayStatics.SetGamePaused` true)
      (else
        (set `/Game/Devices/HackableDevices/Cameras/BP_GameModeCamera.isPaused?` false (`self.Game Mode Camera`))
        (`Widget.RemoveFromParent` (`self.Pause Menu`))
        (`GameplayStatics.SetGamePaused` false)
        (`WidgetBlueprintLibrary.SetInputMode_GameAndUIEx` _returnvalue null)))))

(event `EnhancedInput|/Game/Devices/HackableDevices/Cameras/Inputs/InputActions/IA_Zoom`
  (params (ActionValue :type "Float (double-precision)") (ElapsedSeconds :type "Float (double-precision)") (TriggeredSeconds :type "Float (double-precision)") (InputAction :type "InputAction Object Reference" :default "/Game/Devices/HackableDevices/Cameras/Inputs/InputActions/IA_Zoom.IA_Zoom"))
  (bind _zoomsfx (`self.ZoomSfx`))
  ;[1 1 1] Zoom
  (:`Triggered`
    (bind _camera (`self.GetCamera`))
    (`self.UpdateZoom` _camera ActionValue))
  (:`Started`
    (`AudioComponent.Play` _zoomsfx 0.0)
    (`self.OnZoomInput`))
  (:`Canceled`
    (`AudioComponent.Stop` _zoomsfx :!label _label))
  (:`Completed`
    (goto _label)))

(event `UpdateZoom`
  (params (Camera :type "CameraComponent Object Reference") (ActionValue :type "Float (double-precision)"))
  (bind _zoomvalue (`self.ZoomValue`))
  ;[1 1 1] Zoom
  (bind _output_get (set `self.ZoomValue` (`KismetMathLibrary.FClamp` (+ (`self.ZoomValue`) (/ ActionValue 100.0)) 1.0 (`self.ZoomMax`))))
  (`CameraComponent.SetFieldOfView` Camera (- 90.0 (* (- _output_get 1.0) 30.0)))
  (`/Game/Devices/HackableDevices/Cameras/HUD/WBP_Camera.SetZoomValue` (`self.HUD`) _output_get)
  (if (or (<= _zoomvalue 1.0) (>= _zoomvalue (`self.ZoomMax`)))
    (`AudioComponent.Stop` (`self.ZoomSfx`))))

(fn `BeginPlayActions`
  (`parent.BeginPlayActions`)
  (`|ExecutionSequence`
    (:`then_0`
      ;[1 1 1] BeginPlay : Get controller
      (bind _asplayer_controller (cast `PlayerController` (`self.GetController`)))
      (bind _returnvalue (pcsubsystem `EnhancedInputLocalPlayerSubsystem` _asplayer_controller))
      (`/Engine/EditorBlueprintResources/StandardMacros.IsValid` _returnvalue
        (:`Is Valid`
          (`EnhancedInputSubsystemInterface.AddMappingContext` _returnvalue "/Game/Devices/HackableDevices/Cameras/Inputs/CameraInputs.CameraInputs" 0 (struct))
          (bind _returnvalue_2 (`EnhancedInputSubsystemInterface.GetUserSettings` _returnvalue))
          (if (not (`EnhancedInputUserSettings.IsMappingContextRegistered` _returnvalue_2 "/Game/Devices/HackableDevices/Cameras/Inputs/CameraInputs.CameraInputs"))
            (`EnhancedInputUserSettings.RegisterInputMappingContext` _returnvalue_2 null)))))
    (:`then_1`
      ;[1 1 1] BeginPlay : Set HUD
      (bind _returnvalue_3 (`|CreateWidget` (`self.HUDClass`)))
      (bind _output_get (set `self.HUD` _returnvalue_3))
      (set `Widget.Visibility` "HitTestInvisible" _output_get)
      (`/Game/Devices/HackableDevices/Cameras/HUD/WBP_Camera.SetupHud` _output_get self))
    (:`then_2`
      ;[1 1 1] If default possess
      (if (== self (`GameplayStatics.GetPlayerPawn` 0))
        (`PrimitiveComponent.SetCollisionEnabled` (`self.DetectionBox`) "NoCollision")
        (`UserWidget.AddToViewport` (`self.HUD`) 0)
        (`self.DefaultPossess`)))
    (:`then_3`
      (bind _asbp_game_mode_camera (cast `/Game/Devices/HackableDevices/Cameras/BP_GameModeCamera` (`GameplayStatics.GetGameMode`)))
      (set `self.Game Mode Camera` _asbp_game_mode_camera))))

(fn `ContraintViewModifiers`
  (params (HorizontalModifier :type "Float (double-precision)") (VerticalModifier :type "Float (double-precision)"))
  (returns (NewHorizontalRotation :type "Float (double-precision)") (NewVerticalRotation :type "Float (double-precision)"))
  (locals (NewLocalVar :type "Rotator Structure" :default (struct)))
  (bind (_viewconstraints_ishorizontalconstrained _viewconstraints_horizontalmin _viewconstraints_horizontalmax) (break `/Game/Devices/HackableDevices/Cameras/Struct_ViewConstraints` (`self.ViewConstraints`)))
  (bind (_viewconstraints_ishorizontalconstrained_2 _viewconstraints_horizontalmin_2 _viewconstraints_horizontalmax_2 _viewconstraints_isverticalconstrained _viewconstraints_verticalmin _viewconstraints_verticalmax) (break `/Game/Devices/HackableDevices/Cameras/Struct_ViewConstraints` (`self.ViewConstraints`)))
  (bind (_horizontalrotation _verticalrotation) (`self.GetCameraRotation`))
  (bind _returnvalue (+ HorizontalModifier _horizontalrotation))
  (bind _returnvalue_2 (+ _verticalrotation VerticalModifier))
  (return (select `bool` _viewconstraints_ishorizontalconstrained :`false` _returnvalue :`true` (`KismetMathLibrary.FClamp` _returnvalue (`KismetMathLibrary.Conv_IntToDouble` _viewconstraints_horizontalmin) (`KismetMathLibrary.Conv_IntToDouble` _viewconstraints_horizontalmax))) (select `bool` _viewconstraints_isverticalconstrained :`false` _returnvalue_2 :`true` (`KismetMathLibrary.FClamp` _returnvalue_2 (`KismetMathLibrary.Conv_IntToDouble` _viewconstraints_verticalmin) (`KismetMathLibrary.Conv_IntToDouble` _viewconstraints_verticalmax)))))

(fn `DefaultPossess`
  (bind _game_instance (`self.Game Instance`))
  (bind _returnvalue (`|CreateWidget` "/Game/UI/WBP_AlertScreenOverlay.WBP_AlertScreenOverlay_C"))
  (set `/Game/BP_GameInstance.AlertScreen` _returnvalue _game_instance)
  (bind _returnvalue_2 (`|CreateWidget` "/Game/Text/WBP_Dialog_Box.WBP_Dialog_Box_C"))
  (set `/Game/BP_GameInstance.DialogBox` _returnvalue_2 _game_instance)
  (bind _returnvalue_3 (`|CreateWidget` "/Game/Text/WBP_Popup_Text.WBP_Popup_Text_C"))
  (set `/Game/BP_GameInstance.PopupText` _returnvalue_3 _game_instance)
  (bind _returnvalue_4 (`|CreateWidget` "/Game/Text/WBP_Popup_Alert.WBP_Popup_Alert_C"))
  (set `/Game/BP_GameInstance.PopupAlert` _returnvalue_4 _game_instance))

(fn `GetCamera`
  (returns (Camera :type "CameraComponent Object Reference"))
  (return (`self.Camera`)))

(fn `GetCameraRotation`
  (returns (HorizontalRotation :type "Float (double-precision)") (VerticalRotation :type "Float (double-precision)"))
  (bind _camera (`self.GetCamera`))
  (bind (_relativerotation_roll _relativerotation_pitch _relativerotation_yaw) (`KismetMathLibrary.BreakRotator` (`SceneComponent.RelativeRotation` _camera)))
  (return _relativerotation_yaw _relativerotation_pitch))

(fn `GetRotationModifier`
  (params (Xin :type "Float (double-precision)") (Yin :type "Float (double-precision)"))
  (returns (Xout :type "Float (double-precision)") (Yout :type "Float (double-precision)"))
  (bind _zoomvalue (`self.ZoomValue`))
  (bind _rotationspeedmodifier (`self.RotationSpeedModifier`))
  (return (/ (* Xin _rotationspeedmodifier) _zoomvalue) (/ (* Yin _rotationspeedmodifier) _zoomvalue)))

(fn `Hacked`
  (`parent.Hacked`)
  (bind _asbp_abstract_camera (cast `/Game/Devices/HackableDevices/Cameras/BP_AbstractCamera` (`Controller.K2_GetPawn` (`GameplayStatics.GetPlayerController` 0))))
  (`self.UnpossessCamera` _asbp_abstract_camera)
  (`self.PossessCamera`))

(fn `PossessCamera`
  (`Controller.Possess` (`GameplayStatics.GetPlayerController` 0) self)
  (`/Game/BP_GameInstance.OnPossessedChanged` (`self.Game Instance`))
  (`PrimitiveComponent.SetCollisionEnabled` (`self.DetectionBox`) "NoCollision")
  (`UserWidget.AddToViewport` (`self.HUD`) 0))

(fn `RotateCamera`
  (params (ActionValueX :type "Float (double-precision)") (ActionValueY :type "Float (double-precision)"))
  (bind (_xout _yout) (`self.GetRotationModifier` ActionValueX ActionValueY))
  (bind (_newhorizontalrotation _newverticalrotation) (`self.ContraintViewModifiers` _xout _yout))
  (bind _camera (`self.GetCamera`))
  (`SceneComponent.K2_SetRelativeRotation` _camera (`KismetMathLibrary.MakeRotator` 0.0 _newverticalrotation _newhorizontalrotation) true false))

(fn `UnpossessCamera`
  (`Widget.RemoveFromParent` (`self.HUD`))
  (`PrimitiveComponent.SetCollisionEnabled` (`self.DetectionBox`) "QueryOnly"))

(fn `UserConstructionScript`)