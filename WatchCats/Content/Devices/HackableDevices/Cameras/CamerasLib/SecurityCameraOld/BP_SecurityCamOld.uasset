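; Legacy security camera Blueprint, a hackable device whose view rotates from two-axis input.
; Construction names it "Security Camera" and registers the arm and camera meshes for outlining.
; RotateCamera scales and constrains input through helpers defined outside this file, then yaws the rotator mesh and pitches the camera mesh with inverted sign.
; Getters expose the camera and current rotation; CheckRotation is a debug print, and event graph logic is empty.
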(event `self.ReceiveTick`
  (params (DeltaSeconds :type "Float (single-precision)")))

(fn `CheckRotation`
  (params (CheckName :type String))
  (bind (_relativerotation_roll _relativerotation_pitch) (`KismetMathLibrary.BreakRotator` (`SceneComponent.RelativeRotation` (`self.Camera1`))))
  (if (== _relativerotation_pitch 180.0)
    (`KismetSystemLibrary.PrintString` CheckName true true (struct :`G` 0.694118 :`B` 0.015686 :`A` 1.0))
    (else
      (`KismetSystemLibrary.PrintString` CheckName true true (struct :`R` 1.0 :`B` 0.05137 :`A` 1.0)))))

(fn `GetCamera_0`
  (returns (Camera :type "CameraComponent Object Reference"))
  (return (`self.Camera1`)))

(fn `GetCameraRotation`
  (returns (HorizontalRotation :type "Float (double-precision)") (VerticalRotation :type "Float (double-precision)"))
  (bind (_relativerotation_roll _relativerotation_pitch) (`KismetMathLibrary.BreakRotator` (`SceneComponent.RelativeRotation` (`self.CameraMesh`))))
  (bind (_relativerotation_roll_2 _relativerotation_pitch_2 _relativerotation_yaw) (`KismetMathLibrary.BreakRotator` (`SceneComponent.RelativeRotation` (`self.RotatorMesh`))))
  (return _relativerotation_yaw (* _relativerotation_pitch -1.0)))

(fn `RotateCamera`
  (params (ActionValueX :type "Float (double-precision)") (ActionValueY :type "Float (double-precision)"))
  (bind (_xout _yout) (`self.GetRotationModifier` ActionValueX ActionValueY))
  (bind (_newhorizontalrotation _newverticalrotation) (`self.ContraintViewModifiers` _xout _yout))
  (`SceneComponent.K2_SetRelativeRotation` (`self.RotatorMesh`) (`KismetMathLibrary.MakeRotator` 0.0 0.0 _newhorizontalrotation) true false)
  (`SceneComponent.K2_SetRelativeRotation` (`self.CameraMesh`) (`KismetMathLibrary.MakeRotator` 0.0 (* _newverticalrotation -1.0)) true false))

(fn `UserConstructionScript`
  (`parent.UserConstructionScript`)
  (set `self.MeshToOutline` (`|MakeArray` (`self.ArmMesh`) (`self.CameraMesh`) :!type "MeshComponent Object Reference"))
  (set `self.Name` "Security Camera"))