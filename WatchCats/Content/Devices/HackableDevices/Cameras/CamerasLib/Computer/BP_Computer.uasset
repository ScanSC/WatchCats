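; Hackable computer, built on a possessable camera parent, that gives the player a command terminal to control connected devices.
; Possession shows a camera-swap HUD, and swap functions toggle the WBP_Terminal widget created at BeginPlay.
; Typed input splits into name and parameter, then dispatches to help, clear, list, activate and notes commands.
; Construction randomizes the computer name; two ending commands (download data, destroy virus) exist outside the dispatch switch.
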(event `self.ReceiveBeginPlay`
  (`parent.ReceiveBeginPlay`)
  (`|ExecutionSequence`
    (:`then_0`
      (bind _returnvalue (`|CreateWidget` "/Game/Devices/HackableDevices/Cameras/CamerasLib/Computer/WBP_Terminal.WBP_Terminal_C"))
      (bind _output_get (set `self.Terminal` _returnvalue))
      (set `/Game/Devices/HackableDevices/Cameras/CamerasLib/Computer/WBP_Terminal.Computer` self _output_get))
    (:`then_1`
      (bind _returnvalue_2 (`|CreateWidget` "/Game/Devices/HackableDevices/Cameras/CamerasLib/Computer/WBP_ComputerSwap.WBP_ComputerSwap_C"))
      (set `self.CameraSwapHUD` _returnvalue_2))))

(fn `CommandActivate`
  (params (Parameter :type String))
  (if (`KismetStringLibrary.IsEmpty` Parameter)
    (`/Game/Devices/HackableDevices/Cameras/CamerasLib/Computer/WBP_Terminal.Add_line` (`self.Terminal`) "Usage: Activate <Device_Name>" false)
    (else
      (for _array_element (`self.ConnectedDevices`)
        (if (`KismetStringLibrary.EqualEqual_StrStr` Parameter (`KismetTextLibrary.Conv_TextToString` (`/Game/Devices/ConnectedDevices/BP_AbstractConnectedDevice.Name` _array_element)))
          (`/Game/Devices/ConnectedDevices/BP_AbstractConnectedDevice.Activate` _array_element)
          (`/Game/Devices/HackableDevices/Cameras/CamerasLib/Computer/WBP_Terminal.Add_line` (`self.Terminal`) (`KismetStringLibrary.Concat_StrStr` (`KismetStringLibrary.Concat_StrStr` "Device \"" Parameter) "\" activated.") false)
          (return)
          (else
            (`/Game/Devices/HackableDevices/Cameras/CamerasLib/Computer/WBP_Terminal.Add_line` (`self.Terminal`) (`KismetStringLibrary.Concat_StrStr` (`KismetStringLibrary.Concat_StrStr` "Unkown \"" Parameter) "\" device.") false)))))))

(fn `CommandClear`
  (bind _terminal (`self.Terminal`))
  (`KismetArrayLibrary.Array_Clear` (`/Game/Devices/HackableDevices/Cameras/CamerasLib/Computer/WBP_Terminal.Lines` _terminal))
  (`/Game/Devices/HackableDevices/Cameras/CamerasLib/Computer/WBP_Terminal.Add_line` _terminal "Command lines cleared" false))

(fn `CommandDestroyVirus`
  (bind _asbp_game_instance (cast `/Game/BP_GameInstance` (`GameplayStatics.GetGameInstance`)))
  (`/Game/Text/WBP_Dialog_Box.ShowDialogBox` (`/Game/BP_GameInstance.DialogBox` _asbp_game_instance) 15.0 "Destroying this virus will put an end to the madness of this project. As a friend of mine once said, with great power comes great responsibility.")
  (`Widget.RemoveFromParent` (`self.Terminal`))
  (`PlayerCameraManager.StartCameraFade` :`self` (`GameplayStatics.GetPlayerCameraManager` 0) :`ToAlpha` 1.0 :`Duration` 15.0)
  (set `self.IsFinished` true))

(fn `CommandDownloadData`
  (bind _asbp_game_instance (cast `/Game/BP_GameInstance` (`GameplayStatics.GetGameInstance`)))
  (`/Game/Text/WBP_Dialog_Box.ShowDialogBox` (`/Game/BP_GameInstance.DialogBox` _asbp_game_instance) 5.0 "I didn't know he created something so dangerous, destroying them would be wise.")
  (`Widget.RemoveFromParent` (`self.Terminal`))
  (`PlayerCameraManager.StartCameraFade` :`self` (`GameplayStatics.GetPlayerCameraManager` 0) :`ToAlpha` 1.0 :`Duration` 3.0)
  (set `self.IsFinished` true))

(fn `CommandError`
  (params (CommandName :type String))
  (`/Game/Devices/HackableDevices/Cameras/CamerasLib/Computer/WBP_Terminal.Add_line` (`self.Terminal`) (`KismetStringLibrary.Concat_StrStr` (`KismetStringLibrary.Concat_StrStr` (`KismetStringLibrary.Concat_StrStr` "\"" CommandName) "\"") ": Unrecognized Command. For command list type \"help\".") false))

(fn `CommandHelp`
  (for _array_element (`self.CommandList`)
    (`/Game/Devices/HackableDevices/Cameras/CamerasLib/Computer/WBP_Terminal.Add_line` (`self.Terminal`) (`KismetStringLibrary.Concat_StrStr` (`KismetStringLibrary.Concat_StrStr` (break `/Game/Devices/HackableDevices/Cameras/CamerasLib/Computer/Struct_Commands` _array_element) " : ") (`.Description_8_0473AD014E06234DE09E0E85772B52FC` (break `/Game/Devices/HackableDevices/Cameras/CamerasLib/Computer/Struct_Commands` _array_element))) false)))

(fn `CommandListDevices`
  (if (`KismetArrayLibrary.Array_IsEmpty` (`self.ConnectedDevices`))
    (`/Game/Devices/HackableDevices/Cameras/CamerasLib/Computer/WBP_Terminal.Add_line` (`self.Terminal`) "No connected devices." false)
    (else
      (`/Game/Devices/HackableDevices/Cameras/CamerasLib/Computer/WBP_Terminal.Add_line` (`self.Terminal`) "Connected devices :" false)
      (for _array_element (`self.ConnectedDevices`)
        (`/Engine/EditorBlueprintResources/StandardMacros.IsValid` _array_element
          (:`Is Valid`
            (`/Game/Devices/HackableDevices/Cameras/CamerasLib/Computer/WBP_Terminal.Add_line` (`self.Terminal`) (`KismetTextLibrary.Conv_TextToString` (`/Game/Devices/ConnectedDevices/BP_AbstractConnectedDevice.Name` _array_element)) false)))))))

(fn `CommandNotesMem`
  (`/Game/Devices/HackableDevices/Cameras/CamerasLib/Computer/WBP_Terminal.Add_line` (`self.Terminal`) "Notes memory :" false)
  (`/Game/Devices/HackableDevices/Cameras/CamerasLib/Computer/WBP_Terminal.Add_line` (`self.Terminal`) (`self.NotesMemory`) false))

(fn `Execute Command`
  (params (Command :type String))
  (bind _returnvalue (`KismetStringLibrary.FindSubstring` Command " "))
  (bind _returnvalue_2 (== _returnvalue -1))
  ;[1 1 1] Do nothing if command empty
  (if (not (`KismetStringLibrary.IsEmpty` Command))
    (`self.Manage Command` (select `bool` _returnvalue_2 :`false` (`KismetStringLibrary.Left` Command _returnvalue) :`true` Command) (`KismetStringLibrary.Trim` (select `bool` _returnvalue_2 :`false` (`KismetStringLibrary.RightChop` Command _returnvalue))))))

(fn `GenerateComputerName`
  (bind _output_get (set `self.ComputerName` (`KismetStringLibrary.Concat_StrStr` "Computer " (`KismetStringLibrary.Concat_StrStr` (`KismetStringLibrary.Concat_StrStr` (`KismetStringLibrary.Conv_IntToString` (`KismetMathLibrary.RandomInteger` 9)) (`KismetStringLibrary.Conv_IntToString` (`KismetMathLibrary.RandomInteger` 9))) (`KismetStringLibrary.Concat_StrStr` "." (`KismetStringLibrary.Conv_IntToString` (`KismetMathLibrary.RandomInteger` 9)))))))
  (set `self.Name` (`KismetTextLibrary.Conv_StringToText` _output_get)))

(fn `Manage Command`
  (params (CommandName :type String) (Parameter :type String))
  (`KismetSystemLibrary.PrintString` CommandName)
  (switch `string` CommandName
    (:`Default`
      (`self.CommandError` CommandName))
    (:`help`
      (`self.CommandHelp`))
    (:`Clear`
      (`self.CommandClear`))
    (:`ListDevices`
      (`self.CommandListDevices`))
    (:`Activate`
      (`self.CommandActivate` Parameter))
    (:`NotesMem`
      (`self.CommandNotesMem`))))

(fn `PossessCamera`
  (`parent.PossessCamera`)
  (`UserWidget.AddToViewport` (`self.CameraSwapHUD`) 1))

(fn `SwapToCamera`
  (`Widget.RemoveFromParent` (`self.Terminal`)))

(fn `SwapToTerminal`
  (`UserWidget.AddToViewport` (`self.Terminal`) 0))

(fn `UnpossessCamera`
  (`parent.UnpossessCamera`)
  (`self.SwapToCamera`)
  (`Widget.RemoveFromParent` (`self.CameraSwapHUD`)))

(fn `UserConstructionScript`
  (`parent.UserConstructionScript`)
  (`self.GenerateComputerName`)
  (set `self.MeshToOutline` (`|MakeArray` (`self.Computer`) :!type "MeshComponent Object Reference")))