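; Hackable-camera computer Blueprint that shows a minigame UI when switched to terminal mode.
; On BeginPlay it creates the MiniGame widget, adds it to the viewport and keeps it hidden.
; SwapToTerminal reveals the widget and SwapToCamera hides it again, so one instance is reused by toggling visibility.
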(event `self.ReceiveBeginPlay`
  (`parent.ReceiveBeginPlay`)
  (bind _returnvalue (`|CreateWidget` (`self.MiniGame`)))
  (bind _output_get (set `self.MiniGameWidget` _returnvalue))
  (`UserWidget.AddToViewport` _output_get 1)
  (`Widget.SetVisibility` _output_get "Hidden"))

(fn `SwapToCamera`
  (`Widget.SetVisibility` (`self.MiniGameWidget`) "Hidden"))

(fn `SwapToTerminal`
  (`Widget.SetVisibility` (`self.MiniGameWidget`) "Visible"))

(fn `UserConstructionScript`
  (`parent.UserConstructionScript`))