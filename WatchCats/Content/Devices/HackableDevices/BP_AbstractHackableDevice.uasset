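; Base hackable device that the player hacks by hovering the cursor over it and holding IA_Hold.
; Hover stores the device in BP_GameInstance and applies a hologram overlay to its meshes.
; Holding plays a sound and a timeline driving the hovered device's WBP_Hold bar and a post-process transition material added to the player camera.
; Completion records the device and calls OnHackedDevice on the GameInstance; releasing resets progress.
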(event `self.ReceiveBeginPlay`
  (`self.BeginPlayActions`))

(event `Highlight Object`
  (params (`On/Off` :type Boolean))
  (bind _meshtooutline (`self.MeshToOutline`))
  ;[1 1 1] Highlight object
  (if `On/Off`
    (for _array_element _meshtooutline
      (`MeshComponent.SetOverlayMaterial` _array_element "/Game/Materials/HoverMaterial/MI_Hologram.MI_Hologram"))
    (else
      (for _array_element_2 _meshtooutline
        (`MeshComponent.SetOverlayMaterial` _array_element_2 null)))))

(event `self.DetectionBox.OnBeginCursorOver`
  (params (TouchedComponent :type "PrimitiveComponent Object Reference"))
  (bind _game_instance (`self.Game Instance`))
  ;[1 1 1] On hackable hovered
  (bind _output_get (set `/Game/BP_GameInstance.OveredHackable` self _game_instance))
  (set `/Game/BP_GameInstance.LastOveredHackable` _output_get _game_instance)
  (`self.Highlight Object` true))

(event `self.DetectionBox.OnEndCursorOver`
  (params (TouchedComponent :type "PrimitiveComponent Object Reference"))
  (bind _overedhackable (`/Game/BP_GameInstance.OveredHackable` (`self.Game Instance`)))
  ;[1 1 1] On hackable unhovered
  (`/Engine/EditorBlueprintResources/StandardMacros.IsValid` _overedhackable
    (:`Is Valid`
      (if (== self _overedhackable)
        (set `/Game/BP_GameInstance.OveredHackable` null (`self.Game Instance`) :!label _label)
        (`self.Highlight Object` false)))
    (:`Is Not Valid`
      (goto _label))))

(event `EnhancedInput|/Game/Devices/HackableDevices/Cameras/Inputs/InputActions/IA_Hold`
  (params (ActionValue :type Boolean) (ElapsedSeconds :type "Float (double-precision)") (TriggeredSeconds :type "Float (double-precision)") (InputAction :type "InputAction Object Reference" :default "/Game/Devices/HackableDevices/Cameras/Inputs/InputActions/IA_Hold.IA_Hold"))
  (bind _overedhackable (`/Game/BP_GameInstance.OveredHackable` (`self.Game Instance`)))
  ;[1 1 1] Hack object
  (:`Triggered`
    (`/Engine/EditorBlueprintResources/StandardMacros.IsValid` _overedhackable
      (:`Is Not Valid`
        (`self.StopHacking` :!label _label_2
          (:`ExecOut`
            (bind (_direction _alpha) (`Timeline|Timeline` :!via `Stop` :!label _label_3)
              (:`Update`
                (bind _returnvalue (`KismetMathLibrary.Lerp` 0.0 100.0 _alpha))
                (`self.SetHackingPercentage` _overedhackable _returnvalue)
                (`self.SetTransitionShaderValue` (- 1.0 (/ _returnvalue 100.0))))
              (:`Finished`
                (`self.StopHacking`
                  (:`ExecOut`
                    (`self.Hacked` _overedhackable))))))))))
  (:`Started`
    (`/Engine/EditorBlueprintResources/StandardMacros.IsValid` _overedhackable
      (:`Is Valid`
        (`self.StartHacking`
          (:`ExecOut`
            (goto _label_3 :!via `PlayFromStart`))))))
  (:`Canceled`
    (goto _label_2))
  (:`Completed`
    (goto _label_2)))

(fn `BeginPlayActions`
  (`|ExecutionSequence`
    (:`then_0`
      ;[1 1 1] Get GameInstance
      (bind _asbp_game_instance (cast `/Game/BP_GameInstance` (`GameplayStatics.GetGameInstance`)))
      (set `self.Game Instance` _asbp_game_instance))
    (:`then_1`
      (`self.SetupTransitionShader`))))

(fn `GetCamera`
  (returns (Camera :type "CameraComponent Object Reference"))
  (return (`/Game/Devices/HackableDevices/Cameras/BP_AbstractCamera.Camera` (cast `/Game/Devices/HackableDevices/Cameras/BP_AbstractCamera` (`Controller.K2_GetPawn` (`GameplayStatics.GetPlayerController` 0)) :!pure true))))

(fn `GetInteractMessage`
  (returns (Message :type Text))
  (return (`self.Name`)))

(fn `Hacked`
  (bind _game_instance (`self.Game Instance`))
  (set `/Game/BP_GameInstance.HackedDevice` self _game_instance)
  (`/Game/BP_GameInstance.OnHackedDevice` _game_instance))

(fn `SetHackingPercentage`
  (params (Percentage :type "Float (double-precision)"))
  (bind _output_get (set `self.HackingPercentage` Percentage))
  (bind _aswbp_hold (cast `/Game/Devices/HackableDevices/Cameras/HUD/WBP_Hold` (`WidgetComponent.GetUserWidgetObject` (`self.HackingBar`))))
  (`/Game/Devices/HackableDevices/Cameras/HUD/WBP_Hold.SetPercentage` _aswbp_hold _output_get))

(fn `SetTransitionShaderValue`
  (params (Transition :type "Float (double-precision)" :default 1.0))
  (bind _transitionshader (`self.TransitionShader`))
  (`/Engine/EditorBlueprintResources/StandardMacros.IsValid` _transitionshader
    (:`Is Valid`
      (`MaterialInstanceDynamic.SetScalarParameterValue` _transitionshader "Transition" Transition))))

(fn `SetupTransitionShader`
  (bind _returnvalue (`KismetMaterialLibrary.CreateDynamicMaterialInstance` "/Game/Materials/PostProcess/M_PostProcessHacking.M_PostProcessHacking"))
  (bind _camera (`self.GetCamera`))
  (bind _output_get (set `self.TransitionShader` _returnvalue))
  (`KismetArrayLibrary.Array_Add` (`.Array` (break `WeightedBlendables` (`.WeightedBlendables` (break `PostProcessSettings` (`CameraComponent.PostProcessSettings` _camera))))) (make `WeightedBlendable` 1.0 _output_get))
  (`self.SetTransitionShaderValue` 1.0))

(fn `UserConstructionScript`)