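; BP_AbstractConnectedDevice is a base Blueprint for connected level props that can be toggled and can take codes.
; BeginPlay caches BP_GameInstance, then calls BeginPlayNext, an empty hook for child classes.
; Its Box's cursor-over events set and clear the device as the GameInstance's OveredDevice, without clearing another valid device.
; Activate flips IsActive, while SubmitCode (returns false) and CloseCodePad are stubs.
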(event `self.ReceiveBeginPlay`
  (bind _asbp_game_instance (cast `/Game/BP_GameInstance` (`GameplayStatics.GetGameInstance`)))
  (set `self.Game Instance` _asbp_game_instance)
  (`self.BeginPlayNext`))

(event `BeginPlayNext`)

(event `self.Box.OnBeginCursorOver`
  (params (TouchedComponent :type "PrimitiveComponent Object Reference"))
  (set `/Game/BP_GameInstance.OveredDevice` self (`self.Game Instance`)))

(event `self.Box.OnEndCursorOver`
  (params (TouchedComponent :type "PrimitiveComponent Object Reference"))
  (bind _overeddevice (`/Game/BP_GameInstance.OveredDevice` (`self.Game Instance`)))
  (`/Engine/EditorBlueprintResources/StandardMacros.IsValid` _overeddevice
    (:`Is Valid`
      (if (== self _overeddevice)
        (set `/Game/BP_GameInstance.OveredDevice` null (`self.Game Instance`) :!label _label)))
    (:`Is Not Valid`
      (goto _label))))

(fn `Activate`
  (set `self.isActive` (not (`self.isActive`))))

(fn `CloseCodePad`)

(fn `SubmitCode`
  (params (Code :type String))
  (returns (Success :type Boolean))
  (return false))

(fn `UserConstructionScript`)