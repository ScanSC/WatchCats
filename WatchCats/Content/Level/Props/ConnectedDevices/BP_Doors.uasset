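; A named door prop that slides open or closed as a connected device, with red or green lights showing its state.
; Activate calls the parent, then follows IsActive to run Open or Close, which play or reverse a timeline moving the door block.
; A scene capture feeds a render target and dynamic material into a camera widget, shown on activated opening and removed when the timeline finishes.
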(event `self.ReceiveBeginPlay`
  (`|ExecutionSequence`
    (:`then_0`
      (if (`self.isActive`)
        (`self.Open`)
        (else
          (`self.Close`))))
    (:`then_1`
      ;[1 1 1] Create Camera view
      (bind _returnvalue (`|CreateWidget` "/Game/Level/Props/ConnectedDevices/HUD/WBP_CameraView.WBP_CameraView_C"))
      (set `self.CameraView` _returnvalue))
    (:`then_2`
      ;[1 1 1] Dynamically create a Materialnstance for the widget
      (bind _returnvalue_2 (`KismetRenderingLibrary.CreateRenderTarget2D` 512 512 "RTF_RGBA8"))
      (bind _output_get (set `SceneCaptureComponent2D.TextureTarget` _returnvalue_2 (`self.SceneCaptureComponent2D`)))
      (bind _returnvalue_3 (`KismetMaterialLibrary.CreateDynamicMaterialInstance` "/Game/Level/Props/ConnectedDevices/HUD/M_CameraView.M_CameraView"))
      (bind _output_get_2 (set `self.MaterialInstance` _returnvalue_3))
      (`MaterialInstanceDynamic.SetTextureParameterValue` _output_get_2 "TextInst" _output_get)
      (`/Game/Level/Props/ConnectedDevices/HUD/WBP_CameraView.Set Materiala` (`self.CameraView`) (`self.MaterialInstance`)))))

(event `OpenDoor`
  (bind _doorbloc (`self.DoorBloc`))
  (bind _cameraview (`self.CameraView`))
  (bind (_relativelocation_x _relativelocation_y _relativelocation_z) (`KismetMathLibrary.BreakVector` (`SceneComponent.RelativeLocation` _doorbloc)))
  (bind (_direction _alpha) (`Timeline|OpeningTimeline` :!label _label)
    (:`Update`
      (`SceneComponent.K2_SetRelativeLocation` _doorbloc (`KismetMathLibrary.MakeVector` (`KismetMathLibrary.Lerp` 0.0 -250.0 _alpha) _relativelocation_y _relativelocation_z) false false))
    (:`Finished`
      (`/Engine/EditorBlueprintResources/StandardMacros.IsValid` _cameraview
        (:`Is Valid`
          (`Widget.RemoveFromParent` _cameraview))))))

(event `CloseDoor`
  (goto _label :!via `Reverse`))

(fn `Activate`
  (`parent.Activate`)
  (if (`self.isActive`)
    (`UserWidget.AddToViewport` (`self.CameraView`) 0)
    (`self.Open`)
    (else
      (`self.Close`))))

(fn `Close`
  (set `self.isActive` false)
  (`self.CloseDoor`)
  (`self.UpdateLights`))

(fn `Open`
  (set `self.isActive` true)
  (`self.OpenDoor`)
  (`self.UpdateLights`))

(fn `UpdateLights`
  (if (`self.isActive`)
    (`PrimitiveComponent.SetMaterial` (`self.Cube2`) 0 "/Game/Materials/Mat_GreenBright.Mat_GreenBright")
    (`PrimitiveComponent.SetMaterial` (`self.Cube4`) 0 "/Game/Materials/Mat_GreenBright.Mat_GreenBright")
    (else
      (`PrimitiveComponent.SetMaterial` (`self.Cube2`) 0 "/Game/Materials/Mat_RedBright.Mat_RedBright")
      (`PrimitiveComponent.SetMaterial` (`self.Cube4`) 0 "/Game/Materials/Mat_RedBright.Mat_RedBright"))))

(fn `UserConstructionScript`
  (bind _returnvalue (`KismetTextLibrary.Conv_StringToText` (`self.Name`)))
  (`TextRenderComponent.K2_SetText` (`self.DoorMark1`) _returnvalue)
  (`TextRenderComponent.K2_SetText` (`self.DoorMark2`) _returnvalue))