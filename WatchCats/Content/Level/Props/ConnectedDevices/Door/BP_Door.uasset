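; BP_Door is a connected-device sliding door with colored name marks, red/green state lights and a code pad widget.
; Activate, also triggered by a correct pad code, runs the parent logic, then opens or closes via a timeline according to IsActive.
; Activated opening shows a live camera feed on screen, using a SceneCapture render target and dynamic material, removed shortly after the slide finishes.
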(event `self.BeginPlayNext`
  (`|ExecutionSequence`
    (:`then_0`
      (if (`self.isActive`)
        (`self.Open` null)
        (else
          (`self.Close`))))
    (:`then_1`
      ;[1 1 1] Create Camera view
      (bind _returnvalue (`|CreateWidget` "/Game/Level/Props/ConnectedDevices/HUD/WBP_CameraView.WBP_CameraView_C"))
      (set `self.CameraView` _returnvalue))
    (:`then_2`
      ;[1 1 1] Dynamically create a Materialnstance for the widget
      (bind _returnvalue_2 (`KismetRenderingLibrary.CreateRenderTarget2D` 512 512 "RTF_RGBA8"))
      (bind _output_get (set `SceneCaptureComponent2D.TextureTarget` _returnvalue_2 (`self.SceneCaptureComponent2D`)))
      (bind _returnvalue_3 (`KismetMaterialLibrary.CreateDynamicMaterialInstance` "/Game/Level/Props/ConnectedDevices/HUD/M_CameraView.M_CameraView"))
      (bind _output_get_2 (set `self.MaterialInstance` _returnvalue_3))
      (`MaterialInstanceDynamic.SetTextureParameterValue` _output_get_2 "TextInst" _output_get)
      (`/Game/Level/Props/ConnectedDevices/HUD/WBP_CameraView.Set Materiala` (`self.CameraView`) (`self.MaterialInstance`)))
    (:`then_3`
      ;[1 1 1] Give Itself to WBP_CodePad
      (bind _aswbp_code_pad (cast `/Game/Level/Props/WBP_CodePad` (`WidgetComponent.GetWidget` (`self.CodePad`))))
      (set `/Game/Level/Props/WBP_CodePad.Parent` self _aswbp_code_pad))))

(event `OpenDoor`
  (params (SlideAudio :type "SoundBase Object Reference"))
  (bind _box (`self.Box`))
  (bind _cameraview (`self.CameraView`))
  (bind (_relativelocation_x _relativelocation_y _relativelocation_z) (`KismetMathLibrary.BreakVector` (`SceneComponent.RelativeLocation` _box)))
  (`GameplayStatics.PlaySound2D` SlideAudio 1.0 1.0 0.0 null null)
  (bind (_direction _alpha) (`Timeline|OpeningTimeline` :!label _label)
    (:`Update`
      (`SceneComponent.K2_SetRelativeLocation` _box (`KismetMathLibrary.MakeVector` (`KismetMathLibrary.Lerp` 0.0 -250.0 _alpha) _relativelocation_y _relativelocation_z) false false))
    (:`Finished`
      (`KismetSystemLibrary.Delay` 1.0)
      (`/Engine/EditorBlueprintResources/StandardMacros.IsValid` _cameraview
        (:`Is Valid`
          (`Widget.RemoveFromParent` _cameraview))))))

(event `CloseDoor`
  (goto _label :!via `Reverse`))

(fn `Activate`
  (`parent.Activate`)
  (if (`self.isActive`)
    (`UserWidget.AddToViewport` (`self.CameraView`) 0)
    (`self.Open` "/Game/Level/Props/ConnectedDevices/SFX/slidingDoor.SlidingDoor")
    (else
      (`self.Close`))))

(fn `Close`
  (set `self.isActive` false)
  (`self.CloseDoor`)
  (`self.UpdateLights`))

(fn `CloseCodePad`
  (`SceneComponent.SetVisibility` (`self.CodePad`) false false))

(fn `Open`
  (params (Sound :type "SoundBase Object Reference"))
  (set `self.isActive` true)
  (`self.OpenDoor` Sound)
  (`self.UpdateLights`))

(fn `SubmitCode`
  (params (Code :type String))
  (returns (Success :type Boolean))
  (bind _returnvalue (`SceneComponent.K2_GetComponentLocation` (`self.CodePad`)))
  (if (`KismetStringLibrary.EqualEqual_StrStr` Code (`self.ValidCode`))
    (`GameplayStatics.PlaySoundAtLocation` "/Game/Cameras/CamerasLib/Computer/Audio/Sfx_TerminalOut.Sfx_TerminalOut" _returnvalue (struct) 1.0 1.0 0.0 null null null null)
    (`self.Activate`)
    (return true)
    (else
      (`GameplayStatics.PlaySoundAtLocation` "/Game/Cameras/CamerasLib/Computer/Audio/Sfx_TerminalIn.Sfx_TerminalIn" _returnvalue (struct) 1.0 1.0 0.0 null null null null)
      (return false))))

(fn `UpdateLights`
  (bind _staticmesh1 (`self.StaticMesh1`))
  (bind _staticmesh (`self.StaticMesh`))
  (if (`self.isActive`)
    (`PrimitiveComponent.SetMaterial` _staticmesh 5 "/Game/Materials/Mat_GreenBright.Mat_GreenBright")
    (`PrimitiveComponent.SetMaterial` _staticmesh1 5 "/Game/Materials/Mat_GreenBright.Mat_GreenBright")
    (else
      (`PrimitiveComponent.SetMaterial` _staticmesh 5 "/Game/Materials/Mat_RedBright.Mat_RedBright")
      (`PrimitiveComponent.SetMaterial` _staticmesh1 5 "/Game/Materials/Mat_RedBright.Mat_RedBright"))))

(fn `UserConstructionScript`
  (bind _color (`self.Color`))
  (bind _name (`self.Name`))
  (`|ExecutionSequence`
    (:`then_0`
      (`TextRenderComponent.K2_SetText` (`self.DoorMark1`) _name)
      (`TextRenderComponent.K2_SetText` (`self.DoorMark2`) _name)
      (`TextRenderComponent.SetTextRenderColor` (`self.DoorMark1`) _color)
      (`TextRenderComponent.SetTextRenderColor` (`self.DoorMark2`) _color))))