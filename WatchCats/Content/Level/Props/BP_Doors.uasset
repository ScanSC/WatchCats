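; BP_Doors is a numbered sliding door prop with indicator lights, opened or closed at BeginPlay from IsOpen.
; Open and Close run one timeline forward or in reverse to slide DoorBloc along relative X, then UpdateLights picks green or red materials from IsOpen.
; Close also sets IsOpen to true, so the lights turn green either way.
; The construction script writes Name onto both number marks.
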(event `self.ReceiveBeginPlay`
  (if (`self.isOpen`)
    (`self.Open`)
    (else
      (`self.Close`))))

(event `OpenDoor`
  (bind _doorbloc (`self.DoorBloc`))
  (bind (_relativelocation_x _relativelocation_y _relativelocation_z) (`KismetMathLibrary.BreakVector` (`SceneComponent.RelativeLocation` _doorbloc)))
  (bind (_direction _alpha) (`Timeline|OpeningTimeline` :!label _label)
    (:`Update`
      (`SceneComponent.K2_SetRelativeLocation` _doorbloc (`KismetMathLibrary.MakeVector` (`KismetMathLibrary.Lerp` 0.0 -250.0 _alpha) _relativelocation_y _relativelocation_z) false false))))

(event `CloseDoor`
  (goto _label :!via `Reverse`))

(fn `Close`
  (set `self.isOpen` true)
  (`self.CloseDoor`)
  (`self.UpdateLights`))

(fn `Open`
  (set `self.isOpen` true)
  (`self.OpenDoor`)
  (`self.UpdateLights`))

(fn `UpdateLights`
  (if (`self.isOpen`)
    (`PrimitiveComponent.SetMaterial` (`self.Cube2`) 0 "/Game/Materials/Mat_GreenBright.Mat_GreenBright")
    (`PrimitiveComponent.SetMaterial` (`self.Cube4`) 0 "/Game/Materials/Mat_GreenBright.Mat_GreenBright")
    (else
      (`PrimitiveComponent.SetMaterial` (`self.Cube2`) 0 "/Game/Materials/Mat_RedBright.Mat_RedBright")
      (`PrimitiveComponent.SetMaterial` (`self.Cube4`) 0 "/Game/Materials/Mat_RedBright.Mat_RedBright"))))

(fn `UserConstructionScript`
  (bind _returnvalue (`KismetTextLibrary.Conv_IntToText` (`self.Name`)))
  (`TextRenderComponent.K2_SetText` (`self.NumberMark1`) _returnvalue)
  (`TextRenderComponent.K2_SetText` (`self.NumberMark2`) _returnvalue))